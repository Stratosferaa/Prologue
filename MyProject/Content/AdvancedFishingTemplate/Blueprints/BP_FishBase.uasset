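; Base fish pawn for a fishing system, taking its skeletal mesh from FishProperties.
; An AI MoveTo loop wanders between random navigable points, heads to HookLocation when Attracted, and stops once out of water.
; Until pulled, sighting the player sets the rod's physics-constraint Z limit from their horizontal distance plus slack.
; Tick derives caught and out-of-water flags from InWater, which is not set here.
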(event OnSeePawn(PawnSensing)
  (params (Pawn :type Pawn%20Object%20Reference))
  (bind _rodref (Variables|Default|GetRodRef))
  ;[1 0 0] Getting distance between fish and character to set the rod wire tension
  (if (not (Variables|Default|GetPulled))
    (bind _asbp_fishing_player_character (Utilities|Casting|CastToBP_FishingPlayerCharacter Pawn))
    (Variables|Default|SetCharRef _asbp_fishing_player_character)
    (bind _outhit (Collision|LineTraceByChannel (Transformation|GetActorLocation) (Transformation|GetActorLocation (Variables|Default|GetCharRef)) "TraceTypeQuery1" false 0 "None"))
    (bind _output_get (Variables|Default|SetDistance (Math|Float|Sqrt (+ (Math|Float|Square (.X (Math|Vector|BreakVector (- (.TraceStart (Collision|BreakHitResult _outhit)) (.TraceEnd (Collision|BreakHitResult _outhit)))))) (Math|Float|Square (.Y (Math|Vector|BreakVector (- (.TraceStart (Collision|BreakHitResult _outhit)) (.TraceEnd (Collision|BreakHitResult _outhit))))))))))
    (Utilities|IsValid _rodref
      (:Is%20Valid
        (bind _output_get_2 (Variables|/Game/AdvancedFishingTemplate/Blueprints/BP_FishingRod.BP_FishingRod_C|SetLinearLimit _rodref (+ _output_get 2e+02)))
        (Class|PhysicsConstraintComponent|SetLinearZLimit (Variables|/Game/AdvancedFishingTemplate/Blueprints/BP_FishingRod.BP_FishingRod_C|GetPhysicsConstraint _rodref) "LCM_Limited" _output_get_2)))))

(event EventTick
  (params (DeltaSeconds :type Float%20%28single-precision%29))
  ;[0 1 0] Checking if fish is in water or not
  (if (Variables|Default|GetInWater)
    (Variables|Default|SetFishCaught false)
    (Variables|Default|SetAlreadyOutOfWater false)
    (elif (not (Variables|Default|GetAlreadyOutOfWater))
      (Variables|Default|SetFishCaught true)
      (Variables|Default|SetAlreadyOutOfWater true))))

(event EventBeginPlay
  ;[1 0 0] Fish Moving randomly
  (AI|AIMoveTo self (.RandomLocation (Class|NavigationSystem|GetRandomPointinNavigableRadius (Math|Vector|MakeVector 0.0 0.0 0.0) 2e+03)) 0 0.0 false :!label _label
    (:OnSuccess
      _)
    (:OnFail
      _))
  (Utilities|FlowControl|Delay 0.2 :!label _label_2)
  ;[1 0 0] Checking if fish is in the water or not
  (if (Variables|Default|GetInWater)
    ;[1 0 0] Checking if fish is attracted to hook
    (if (not (Variables|Default|GetAttracted))
      (goto _label)
      (else
        ;[1 0 0] Atracted to food, now move towards hook
        (AI|AIMoveTo self (Variables|Default|GetHookLocation) 0 0.0 false
          (:OnSuccess
            (Variables|Default|SetAttracted false)
            (goto _label_2)))))
    (else
      ;[1 0 0] If fish is out of water stop movement
      (Components|Movement|StopMovementImmediately (Variables|Character|GetCharacterMovement)))))

(fn ConstructionScript
  (Class|SkinnedMeshComponent|SetSkeletalMesh (Variables|Character|GetMesh) (.Mesh (Utilities|Struct|BreakFishDetails (Variables|Default|GetFishProperties))) true))