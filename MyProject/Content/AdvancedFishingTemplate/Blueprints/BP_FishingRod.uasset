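; Fishing rod actor that casts a hook on a physics-constraint line, attracts fish and hooks one on contact.
; Cast and reel events set the constraint's Z limit through gated delay loops, with heavier fish reeling up slower.
; Overlap volumes lure fish and record the catch.
; Tick then swaps attachment: fish follows the physics hook while the player reels up, otherwise the hook follows the fish in water.
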(event OnComponentBeginOverlap(HookVolume)
  (params (OverlappedComponent :type Primitive%20Component%20Object%20Reference) (OtherActor :type Actor%20Object%20Reference) (OtherComp :type Primitive%20Component%20Object%20Reference) (OtherBodyIndex :type Integer) (bFromSweep :type Boolean) (SweepResult :type Hit%20Result%20Structure%20%28by%20ref%29))
  ;[1 0 0] Fish Caught
  (if (not (Variables|Default|GetCaught))
    (bind _asbp_fish_base (Utilities|Casting|CastToBP_FishBase OtherActor))
    (Variables|Default|SetCurrentFishRef _asbp_fish_base)
    (Variables|/Game/AdvancedFishingTemplate/Blueprints/BP_FishBase.BP_FishBase_C|SetRodRef _asbp_fish_base self)
    (Variables|Default|SetCaught true)))

(event OnComponentBeginOverlap(AttractionVolume)
  (params (OverlappedComponent :type Primitive%20Component%20Object%20Reference) (OtherActor :type Actor%20Object%20Reference) (OtherComp :type Primitive%20Component%20Object%20Reference) (OtherBodyIndex :type Integer) (bFromSweep :type Boolean) (SweepResult :type Hit%20Result%20Structure%20%28by%20ref%29))
  ;[1 0 0] Fish Attracted towards hook
  (bind _asbp_fish_base (Utilities|Casting|CastToBP_FishBase OtherActor))
  (Variables|/Game/AdvancedFishingTemplate/Blueprints/BP_FishBase.BP_FishBase_C|SetAttracted _asbp_fish_base true)
  (Variables|/Game/AdvancedFishingTemplate/Blueprints/BP_FishBase.BP_FishBase_C|SetHookLocation _asbp_fish_base (Transformation|GetWorldLocation (Variables|Default|Gethook))))

(event Custom|ReelDown
  ;[1 0 0] Reel Down
  (Utilities|FlowControl|Sequence
    (:then_0
      (goto _label Open))
    (:then_1
      (Utilities|FlowControl|Gate true :!label _label
        (:Exit
          (bind _output_get (Variables|Default|SetLinearLimit (+ (Variables|Default|GetLinearLimit) 2.0)))
          (Class|PhysicsConstraintComponent|SetLinearZLimit (Variables|Default|GetPhysicsConstraint) "LCM_Limited" _output_get)
          (Utilities|FlowControl|Delay 0.01)
          (goto _label))))))

(event Custom|ReelDownStop
  ;[1 0 0] Reel Down
  (Utilities|FlowControl|Gate true) ; enters at Close
)

(event Custom|ReelUpStop
  (bind _physicsconstraint (Variables|Default|GetPhysicsConstraint))
  (bind _currentfishref (Variables|Default|GetCurrentFishRef))
  (bind _fishproperties (Variables|/Game/AdvancedFishingTemplate/Blueprints/BP_FishBase.BP_FishBase_C|GetFishProperties _currentfishref))
  (bind _weight (Utilities|Struct|BreakFishDetails _fishproperties))
  ;[1 0 0] Reel Up
  (Utilities|FlowControl|Gate true) ; enters at Close
)

(event Custom|ReelUp
  (bind _physicsconstraint (Variables|Default|GetPhysicsConstraint))
  (bind _currentfishref (Variables|Default|GetCurrentFishRef))
  (bind _fishproperties (Variables|/Game/AdvancedFishingTemplate/Blueprints/BP_FishBase.BP_FishBase_C|GetFishProperties _currentfishref))
  (bind _weight (Utilities|Struct|BreakFishDetails _fishproperties))
  ;[1 0 0] Reel Up
  (Utilities|FlowControl|Sequence
    (:then_0
      (goto _label Open))
    (:then_1
      (Utilities|FlowControl|Gate true :!label _label
        (:Exit
          ;;[0.1431 1 0] ReelingSpeed Depending on fish weight
          (Utilities|IsValid _currentfishref
            (:Is%20Valid
              (if (> _weight 1.0)
                (bind _output_get (Variables|Default|SetLinearLimit (+ (Variables|Default|GetLinearLimit) (/ -3.0 _weight))))
                (Class|PhysicsConstraintComponent|SetLinearZLimit _physicsconstraint "LCM_Limited" _output_get)
                (else
                  (bind _output_get_2 (Variables|Default|SetLinearLimit (+ (Variables|Default|GetLinearLimit) -3.0) :!label _label_2))
                  (Class|PhysicsConstraintComponent|SetLinearZLimit _physicsconstraint "LCM_Limited" _output_get_2))))
            (:Is%20Not%20Valid
              (goto _label_2)))
          (Utilities|FlowControl|Delay 0.01)
          (goto _label))))))

(event Custom|Cast
  ;[1 0 0] Cast
  (bind _output_get (Variables|Default|SetLinearLimit 1e+03))
  (Class|PhysicsConstraintComponent|SetLinearZLimit (Variables|Default|GetPhysicsConstraint) "LCM_Limited" _output_get))

(event EventTick
  (params (DeltaSeconds :type Float%20%28single-precision%29))
  (bind _hook (Variables|Default|Gethook))
  (bind _currentfishref (Variables|Default|GetCurrentFishRef))
  (bind _currentfishref_2 (Variables|Default|GetCurrentFishRef))
  (bind _hook_2 (Variables|Default|Gethook))
  (bind _hook_3 (Variables|Default|Gethook))
  (bind _rootcomponent (Variables|/Script/Engine.Actor|GetRootComponent _currentfishref_2))
  ;[0 1 0] Tick is deciding weather hook should be parent or fish
  (if (Variables|Default|GetCaught)
    (if (Variables|/Game/AdvancedFishingTemplate/Blueprints/BP_FishingPlayerCharacter.BP_FishingPlayerCharacter_C|GetReelUp (Variables|Default|GetCharRef))
      (if (not (Variables|Default|GetHookParent))
        (Variables|/Game/AdvancedFishingTemplate/Blueprints/BP_FishBase.BP_FishBase_C|SetPulled _currentfishref true)
        (Collision|SetCollisionEnabled _hook_2 "QueryAndPhysics")
        (Transformation|DetachFromComponent _hook_2 "KeepWorld" "KeepWorld" "KeepWorld" true)
        (Transformation|AttachComponentToComponent _rootcomponent _hook "hook" "SnapToTarget" "SnapToTarget" "KeepWorld" true)
        (Physics|SetSimulatePhysics _hook true)
        (Variables|Default|SetHookParent true)
        (Variables|Default|SetFishParent false))
      (elif (not (Variables|Default|GetFishParent))
        (if (Variables|/Game/AdvancedFishingTemplate/Blueprints/BP_FishBase.BP_FishBase_C|GetInWater (Variables|Default|GetCurrentFishRef))
          (Variables|/Game/AdvancedFishingTemplate/Blueprints/BP_FishBase.BP_FishBase_C|SetPulled (Variables|Default|GetCurrentFishRef) false)
          (Transformation|DetachFromComponent (Variables|/Script/Engine.Actor|GetRootComponent _currentfishref) "KeepWorld" "KeepWorld" "KeepWorld" true)
          (Transformation|AttachComponentToComponent _hook_3 _rootcomponent "test" "SnapToTarget" "SnapToTarget" "KeepWorld" true)
          (Physics|SetSimulatePhysics _hook_3 false)
          (Collision|SetCollisionEnabled _hook_3 "PhysicsOnly")
          (Variables|Default|SetFishParent true)
          (Variables|Default|SetHookParent false))))))

(event EventBeginPlay
  ;[0 0 1] Taking Character Ref
  (bind _asbp_fishing_player_character (Utilities|Casting|CastToBP_FishingPlayerCharacter (Game|GetPlayerCharacter 0)))
  (Variables|Default|SetCharRef _asbp_fishing_player_character))

(fn ConstructionScript)