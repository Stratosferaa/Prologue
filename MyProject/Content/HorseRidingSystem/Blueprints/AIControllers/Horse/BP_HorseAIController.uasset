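; AI controller for horses that runs the horse behavior tree and makes them come to a whistle and kick behind them.
; Hearing perception puts the whistler on the Blackboard, except for follower horses, and sets speed by distance.
; Tick slows the horse nearby and clears detection after arrival.
; A delayed, repeated rear line trace triggers the kick montage, knocking back the third-person character with a snort; path-following code is left unwired.
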(event OnTargetPerceptionUpdated(AIPerception_hearing)
  (params (Actor :type Actor%20Object%20Reference) (Stimulus :type AI%20Stimulus%20Structure))
  (bind _returnvalue (Pawn|GetControlledPawn))
  (bind _returnvalue_2 (Pawn|GetControlledPawn))
  (if (not (.bSuccess (Utilities|Casting|CastToBP_Horse_Follower _returnvalue_2)))
    (bind _output_get (Variables|Default|SetWhistledActor Actor))
    (if (.bsuccessfullysensed Stimulus)
      (Class|BlackboardComponent|SetValueasInt (AI|GetBlackboard 0) (Utilities|Name|MakeLiteralName "Detection State") 1)
      (bind _output_get_2 (Variables|Default|SetLengthToWhistleLocation (Class|KismetMathLibrary|Hypotenuse (.x (- (Transformation|GetActorLocation _output_get) (Transformation|GetActorLocation _returnvalue_2))) (.y (- (Transformation|GetActorLocation _output_get) (Transformation|GetActorLocation _returnvalue_2))))))
      (if (> _output_get_2 2e+03)
        (Class|BPIHorseAI|SetMaxWalkSpeed(Message) _returnvalue 1e+03)
        (else
          (Class|BPIHorseAI|SetMaxWalkSpeed(Message) _returnvalue 2e+02)))
      (AI|Components|Blackboard|SetValueasObject (AI|GetBlackboard 0) (Utilities|Name|MakeLiteralName "PlayerObj") (Variables|Default|GetWhistledActor)))))

(event EventBeginPlay
  (AI|RunBehaviorTree "/Game/HorseRidingSystem/Blueprints/AIControllers/Horse/BT_Horse.BT_Horse")
  (Class|AIController|UseBlackboard "/Game/HorseRidingSystem/Blueprints/AIControllers/Horse/BB_Horse.BB_Horse")
  (bind _asbp_horse (Utilities|Casting|CastToBP_Horse (Pawn|GetControlledPawn)))
  (Variables|Default|SetMainHorse _asbp_horse))

(event EventTick
  (params (DeltaSeconds :type Float%20%28single-precision%29))
  (bind _returnvalue (Pawn|GetControlledPawn))
  (bind _mainhorse (Variables|Default|GetMainHorse))
  (bind _whistledactor (Variables|Default|GetWhistledActor))
  (bind _returnvalue_2 (Transformation|GetActorLocation _whistledactor))
  (bind _returnvalue_3 (Transformation|GetActorLocation _returnvalue))
  (bind _mesh (Variables|/Script/Engine.Character|GetMesh _mainhorse))
  (bind _returnvalue_4 (Transformation|GetSocketLocation _mesh "Toe_Left"))
  (bind _returnvalue_5 (- _returnvalue_2 _returnvalue_3))
  (bind _returnvalue_6 (Math|Vector|VectorLength _returnvalue_5))
  ;[1 1 1] Stop player following part
  (Utilities|FlowControl|Sequence
    (:then_0
      (Utilities|IsValid _whistledactor
        (:Is%20Valid
          (Utilities|IsValid _returnvalue
            (:Is%20Valid
              (if (< _returnvalue_6 3e+02)
                (Utilities|FlowControl|Delay 1e+01)
                (Class|BlackboardComponent|SetValueasInt (AI|GetBlackboard 0) (Utilities|Name|MakeLiteralName "Detection State"))
                (elif (< _returnvalue_6 7e+02)
                  (Class|BPIHorseAI|SetMaxWalkSpeed(Message) (Pawn|GetControlledPawn) 2e+02))))))))
    (:then_1
      (bind _returnvalue_7 (CallFunction|BackLineTrace -1.2e+02))
      (if _returnvalue_7
        (Utilities|FlowControl|Delay 5.0)
        (bind (_returnvalue_8 _outhit) (CallFunction|BackLineTrace -1.2e+02))
        (if _returnvalue_8
          (Animation|Montage|PlayMontage (Variables|/Script/Engine.Character|GetMesh (Variables|Default|GetMainHorse)) "/Game/HorseRidingSystem/Animations/AM_HorseBack_kick.AM_HorseBack_kick"
            (:then
              (if (Utilities|Enum|Equal(Enum) (Utilities|GetDisplayName (.HitActor (Collision|BreakHitResult _outhit))) "BP_ThirdPersonCharacter")
                (Audio|PlaySoundatLocation "/Game/HorseRidingSystem/Audio/Snort/SC_HorseSnort_Cue.SC_HorseSnort_Cue" (Transformation|GetSocketLocation (Variables|/Script/Engine.Character|GetMesh (Variables|Default|GetMainHorse)) "head") "0, 0, 0" 1.0 1.0 0.0 0 0 0)
                (Utilities|FlowControl|Delay 1.0)
                (Default|HorseKick (.AsBP%20Third%20Person%20Character (Utilities|Casting|CastToBP_ThirdPersonCharacter (.HitActor (Collision|BreakHitResult _outhit)))) (- _returnvalue_4 (+ _returnvalue_4 (* (Math|Vector|GetForwardVector (Transformation|GetSocketRotation _mesh "Toe_Left")) -8e+02))))))))))
    (:then_2
      (if (== (Class|BlackboardComponent|GetValueasInt (AI|GetBlackboard 0) (Utilities|Name|MakeLiteralName "Detection State")) 0)
        _))))

(fn ConstructionScript)

(fn BackLineTrace
  (params (B :type Float%20%28single-precision%29))
  (bind _mainhorse (Variables|Default|GetMainHorse))
  (bind _mesh (Variables|/Script/Engine.Character|GetMesh _mainhorse))
  (bind _returnvalue (Transformation|GetSocketLocation _mesh "Pelvis"))
  (Utilities|IsValid _mainhorse
    (:Is%20Valid
      (bind (_outhit _returnvalue_2) (Collision|LineTraceByChannel (+ (* (Transformation|GetActorForwardVector _mainhorse) -2e+01) _returnvalue) (+ _returnvalue (* (Transformation|GetActorForwardVector _mainhorse) B)) "TraceTypeQuery1" true 0 "None"))
      (return _returnvalue_2 _outhit))))

(fn GetMoveLocation
  (return "0, 0, 0"))