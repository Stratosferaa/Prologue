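; Horse actor that follows the spline of a referenced track, starting on BeginPlay when ActiveFollowing is set.
; A timeline, with play rate set from Duration and start time from HorseStartOffset, maps its alpha to distance along the spline.
; Each update takes XY and rotation from the spline, keeps the actor's own Z, and feeds a fixed forward speed to the BPA_horse animation instance.
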(event Custom|Move%20Horse
  (Components|Timeline|SetPlayRate (Variables|Default|GetHorseFollow) (/ 1.0 (Variables|Default|GetDuration)))
  (Components|Timeline|SetNewTime (Variables|Default|GetHorseFollow) (Variables|Default|GetHorseStartOffset))
  (bind _alpha (Timeline|HorseFollow Play)
    (:Update
      (Variables|Default|SetAlpha _alpha)
      (Variables|/Game/HorseRidingSystem/Blueprints/BPA_horse.BPA_horse_C|SetSpeed%20Forward (.AsBPA%20Horse (Utilities|Casting|CastToBPA_horse (Components|SkeletalMesh|GetAnimInstance (Variables|Character|GetMesh)))) 1e+03)
      (Transformation|SetActorLocationAndRotation (Math|Vector|MakeVector (.x (Spline|GetLocationatDistanceAlongSpline (Variables|/Game/HorseRidingSystem/Blueprints/RunningPath.RunningPath_C|GetPathSpline (Variables|Default|GetTrackRef)) (Math|Float|Lerp 0.0 (Spline|GetSplineLength (Variables|/Game/HorseRidingSystem/Blueprints/RunningPath.RunningPath_C|GetPathSpline (Variables|Default|GetTrackRef))) (Variables|Default|GetAlpha)) "World")) (.y (Spline|GetLocationatDistanceAlongSpline (Variables|/Game/HorseRidingSystem/Blueprints/RunningPath.RunningPath_C|GetPathSpline (Variables|Default|GetTrackRef)) (Math|Float|Lerp 0.0 (Spline|GetSplineLength (Variables|/Game/HorseRidingSystem/Blueprints/RunningPath.RunningPath_C|GetPathSpline (Variables|Default|GetTrackRef))) (Variables|Default|GetAlpha)) "World")) (.z (Transformation|GetActorLocation))) (Spline|GetRotationatDistanceAlongSpline (Variables|/Game/HorseRidingSystem/Blueprints/RunningPath.RunningPath_C|GetPathSpline (Variables|Default|GetTrackRef)) (Math|Float|Lerp 0.0 (Spline|GetSplineLength (Variables|/Game/HorseRidingSystem/Blueprints/RunningPath.RunningPath_C|GetPathSpline (Variables|Default|GetTrackRef))) (Variables|Default|GetAlpha)) "World")))))

(event EventBeginPlay
  (|CallParentFunction)
  (if (Variables|Default|GetActiveFollowing?)
    (CallFunction|MOveHorse)))

(event Collision|EventActorBeginOverlap
  (params (OtherActor :type Actor%20Object%20Reference))
  (|CallParentFunction OtherActor) ; This node is disabled and will not be called.\nDrag off pins to build functionality.
)

(event EventTick
  (params (DeltaSeconds :type Float%20%28single-precision%29))
  (|CallParentFunction DeltaSeconds) ; This node is disabled and will not be called.\nDrag off pins to build functionality.
)

(fn ConstructionScript
  (|CallParentFunction))