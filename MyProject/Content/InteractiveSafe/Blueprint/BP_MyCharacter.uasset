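; First-person player character for an interactive safe feature, with Enhanced Input movement, look and interaction.
; Each tick, a camera line trace caches the hit actor and component, and the pointer widget reflects whether that component is in range and tagged "Useable".
; Interact rechecks the cached hit, passing zero distance, and sends InteractMessage with the component to the actor.
; BeginPlay displays the pointer widget and creates, without displaying, a safe number widget.
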(event Input|EnhancedActionEvents|EnhancedInputActionIA_MoveY
  (params (ActionValue :type Float%20%28double-precision%29) (ElapsedSeconds :type Float%20%28double-precision%29) (TriggeredSeconds :type Float%20%28double-precision%29) (InputAction :type Input%20Action%20Object%20Reference :default "/Game/InteractiveSafe/Input/IA_MoveY.IA_MoveY"))
  ;[1 0.4452 0] WASD Movement
  (:Triggered
    (Pawn|Input|AddMovementInput (Transformation|GetActorForwardVector) ActionValue false)))

(event Input|EnhancedActionEvents|EnhancedInputActionIA_MoveX
  (params (ActionValue :type Float%20%28double-precision%29) (ElapsedSeconds :type Float%20%28double-precision%29) (TriggeredSeconds :type Float%20%28double-precision%29) (InputAction :type Input%20Action%20Object%20Reference :default "/Game/InteractiveSafe/Input/IA_MoveX.IA_MoveX"))
  ;[1 0.4452 0] WASD Movement
  (:Triggered
    (Pawn|Input|AddMovementInput (Transformation|GetActorRightVector) ActionValue false)))

(event Input|EnhancedActionEvents|EnhancedInputActionIA_LookX
  (params (ActionValue :type Float%20%28double-precision%29) (ElapsedSeconds :type Float%20%28double-precision%29) (TriggeredSeconds :type Float%20%28double-precision%29) (InputAction :type Input%20Action%20Object%20Reference :default "/Game/InteractiveSafe/Input/IA_LookX.IA_LookX"))
  ;[1 0.4452 0] Look Arround
  (:Triggered
    (Pawn|Input|AddControllerYawInput ActionValue)))

(event Input|EnhancedActionEvents|EnhancedInputActionIA_LookY
  (params (ActionValue :type Float%20%28double-precision%29) (ElapsedSeconds :type Float%20%28double-precision%29) (TriggeredSeconds :type Float%20%28double-precision%29) (InputAction :type Input%20Action%20Object%20Reference :default "/Game/InteractiveSafe/Input/IA_LookY.IA_LookY"))
  ;[1 0.4452 0] Look Arround
  (:Triggered
    (Pawn|Input|AddControllerPitchInput ActionValue)))

(event Input|EnhancedActionEvents|EnhancedInputActionIA_Interact
  (params (ActionValue :type Boolean) (ElapsedSeconds :type Float%20%28double-precision%29) (TriggeredSeconds :type Float%20%28double-precision%29) (InputAction :type Input%20Action%20Object%20Reference :default "/Game/InteractiveSafe/Input/IA_Interact.IA_Interact"))
  ;[1 0.4452 0] Interact
  (:Triggered
    (bind _useable (CallFunction|CheckTraceActor 0.0))
    (if _useable
      (Class|BPInteractInterface|Interact(Message) (Variables|LineTrace|GetHit%20Actor) (Variables|LineTrace|GetHit%20Component)))))

(event EventTick
  (params (DeltaSeconds :type Float%20%28single-precision%29))
  ;[1 1 1] LineTrace and Change Pointer
  (bind (_hitactor _hitcomponent _distance) (CallFunction|LineTrace))
  (Variables|LineTrace|SetHit%20Actor _hitactor)
  (Variables|LineTrace|SetHit%20Component _hitcomponent)
  (bind _useable (CallFunction|CheckTraceActor _distance))
  (Default|ChangePointer (Variables|Widgets|GetPointer%20Widget) (Variables|Default|GetRemove%20All%20Pointer) _useable))

(event EventBeginPlay
  ;[1 1 1] Create Widgets
  (bind _returnvalue (UserInterface|CreateWidget "/Game/InteractiveSafe/Widgets/WB_PointerWidget.WB_PointerWidget_C"))
  (bind _output_get (Variables|Widgets|SetPointer%20Widget _returnvalue))
  (UserInterface|Viewport|AddtoViewport _output_get 0)
  (bind _returnvalue_2 (UserInterface|CreateWidget "/Game/InteractiveSafe/Widgets/WB_SafeNumberWidget.WB_SafeNumberWidget_C"))
  (Variables|Widgets|SetSafeNumber%20Widget _returnvalue_2))

(fn ConstructionScript)

(fn LineTrace
  (bind _camera (Variables|Default|GetCamera))
  (bind _returnvalue (Transformation|GetWorldLocation _camera))
  (bind (_outhit _returnvalue_2) (Collision|LineTraceByChannel _returnvalue (+ _returnvalue (* (Math|Vector|GetForwardVector _camera) (Variables|Default|GetMax%20Use%20Distance))) "TraceTypeQuery1" false 0 "None"))
  (if _returnvalue_2
    (return (.HitActor (Collision|BreakHitResult _outhit)) (.HitComponent (Collision|BreakHitResult _outhit)) (.Distance (Collision|BreakHitResult _outhit)))
    (else
      (return 0 0 (.Distance (Collision|BreakHitResult _outhit))))))

(fn CheckTraceActor
  (params (Distance :type Float%20%28double-precision%29))
  (bind _hit_actor (Variables|LineTrace|GetHit%20Actor))
  (Utilities|IsValid _hit_actor
    (:Is%20Valid
      (return (Math|Boolean|ANDBoolean (Utilities|IsValid _hit_actor) (Components|ComponentHasTag (Variables|LineTrace|GetHit%20Component) "Useable") (< Distance (Variables|Default|GetMax%20Use%20Distance)))))
    (:Is%20Not%20Valid
      (return false))))