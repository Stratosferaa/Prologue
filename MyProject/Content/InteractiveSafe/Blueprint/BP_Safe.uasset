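; Interactive safe with a combination dial and handle that the player cracks to open the door.
; Using the dial blends the view to the safe and moves input to it, showing the current number in a widget.
; Each timeline-driven spin converts roll to a number, records it with its direction and compares the sequence to the combination.
; A match unlocks, removes "Useable" tags and returns control, opening automatically if AutoOpen or via the handle.
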(event Custom|Open%20Safe
  ;[0 0.9911 1] Open Safe
  (CallFunction|HandleAnimation (Variables|Settings|GetLocked))
  (Utilities|FlowControl|Delay 1.6)
  (CallFunction|DoorAnimation)
  (CallFunction|DeactivateUseable (Variables|Default|GetSafe_Door_Handle) "Useable"))

(event Custom|Handle%20Interacted
  ;[1 1 1] Handle Interacted
  (if (Variables|Settings|GetLocked)
    (CallFunction|HandleAnimation (Variables|Settings|GetLocked))
    (else
      (CallFunction|OpenSafe))))

(event Custom|Door%20Animation
  ;[0 0.9911 1] Door Animation
  (Utilities|FlowControl|DoOnce false :!label _label
    (:Completed
      (bind _alpha (Timeline|DoorAnimationTimeline PlayFromStart)
        (:Update
          (Transformation|SetRelativeRotation (Variables|Default|GetSafe_Door) (Math|Rotator|MakeRotator 0.0 0.0 (Math|Float|Lerp 0.0 (Variables|Settings|GetDoor%20Open%20Angle) _alpha)) false false))
        (:Finished
          (goto _label Reset))
        (:Open%20Sound
          (CallFunction|DoorOpenSound))))))

(event Custom|Handle%20Animation
  (params (Locked? :type Boolean))
  ;[0 0.9911 1] Handle Animation
  (Utilities|FlowControl|DoOnce false :!label _label
    (:Completed
      (bind (_direction _locked_y _open_y) (Timeline|HandleAnimationTimeline PlayFromStart)
        (:Update
          (Transformation|SetRelativeRotation (Variables|Default|GetSafe_Door_Handle) (Math|Rotator|MakeRotator (Math|Float|SelectFloat _locked_y _open_y Locked?) 0.0 0.0) false false))
        (:Finished
          (goto _label Reset))
        (:Locked%20Sound
          (if Locked?
            (CallFunction|HandleSound Locked?)))
        (:Open%20Sound
          (if (not Locked?)
            (CallFunction|HandleSound Locked?)))))))

(event Custom|Handle%20Sound
  (params (Locked :type Boolean))
  ;[0.8879 0 1] SOUNDS
  (if Locked
    (Audio|PlaySound2D "/Game/InteractiveSafe/Audio/SC_Handle_Locked.SC_Handle_Locked" 1.0 1.0 0.0 0 0)
    (else
      (Audio|PlaySound2D "/Game/InteractiveSafe/Audio/SC_MetalOpen.SC_MetalOpen" 1.0 1.0 0.0 0 0))))

(event Custom|Lock%20Spin%20Sound
  ;[0.8879 0 1] SOUNDS
  (Audio|PlaySound2D "/Game/InteractiveSafe/Audio/SC_MechanicalKey.SC_MechanicalKey" 1.0 1.0 0.0 0 0))

(event Custom|Door%20Open%20Sound
  ;[0.8879 0 1] SOUNDS
  (Audio|PlaySound2D "/Game/InteractiveSafe/Audio/SC_MetalCreak.SC_MetalCreak" 1.0 1.0 0.0 0 0))

(event Custom|Give%20input%20to%20Safe
  (bind _returnvalue (Game|GetPlayerController 0))
  (bind _as_my_character (Variables|Default|GetAs%20My%20Character))
  (bind _safenumber_widget (Variables|/Game/InteractiveSafe/Blueprint/BP_MyCharacter.BP_MyCharacter_C|GetSafeNumber%20Widget _as_my_character))
  ;[1 1 1] Give Input to Safe
  (Variables|/Game/InteractiveSafe/Blueprint/BP_MyCharacter.BP_MyCharacter_C|SetRemove%20All%20Pointer (Variables|Default|GetAs%20My%20Character) true)
  (Input|DisableInput (Variables|Default|GetAs%20My%20Character) _returnvalue)
  (Game|Player|SetViewTargetwithBlend _returnvalue self 1.6 "VTBlend_Cubic" 1.0 false)
  (Utilities|FlowControl|Delay 1.6)
  (Input|EnableInput (Game|GetPlayerController 0))
  (UserInterface|Viewport|AddtoViewport _safenumber_widget 0)
  (Variables|/Game/InteractiveSafe/Widgets/WB_SafeNumberWidget.WB_SafeNumberWidget_C|SetSafeNumber _safenumber_widget (Utilities|Text|ToText(String) (Variables|SafeCombination|GetSelected%20Number))))

(event Custom|Give%20input%20to%20Player
  (bind _returnvalue (Game|GetPlayerController 0))
  ;[1 1 1] Give Input to Player
  (Widget|RemovefromParent (Variables|/Game/InteractiveSafe/Blueprint/BP_MyCharacter.BP_MyCharacter_C|GetSafeNumber%20Widget (Variables|Default|GetAs%20My%20Character)))
  (Input|DisableInput _returnvalue)
  (Game|Player|SetViewTargetwithBlend _returnvalue (Variables|Default|GetAs%20My%20Character) 1.6 "VTBlend_Cubic" 1.0 false)
  (Utilities|FlowControl|Delay 1.6)
  (Input|EnableInput (Variables|Default|GetAs%20My%20Character) (Game|GetPlayerController 0))
  (Variables|/Game/InteractiveSafe/Blueprint/BP_MyCharacter.BP_MyCharacter_C|SetRemove%20All%20Pointer (Variables|Default|GetAs%20My%20Character) false))

(event Custom|Lock%20Rotation
  (params (Direction :type Float%20%28double-precision%29))
  ;[1 0 0] Lock Rotation
  (Variables|LockAnimation|SetDirection Direction)
  (Utilities|FlowControl|DoOnce false :!label _label
    (:Completed
      (Variables|LockAnimation|SetDesired%20Rotation (* Direction (Variables|Settings|GetSpin%20Tick%20Degree)))
      (Variables|LockAnimation|SetLock%20Rotation%20X (.roll (Variables|/Script/Engine.SceneComponent|GetRelativeRotation (Variables|Default|GetSafe_Door_Lock))))
      (bind _alpha (Timeline|LockRotationTimer PlayFromStart)
        (:Update
          (Transformation|SetRelativeRotation (Variables|Default|GetSafe_Door_Lock) (Math|Rotator|MakeRotator (Math|Float|Lerp (Variables|LockAnimation|GetLock%20Rotation%20X) (+ (Variables|LockAnimation|GetLock%20Rotation%20X) (Variables|LockAnimation|GetDesired%20Rotation)) _alpha) 0.0 0.0) false false))
        (:Finished
          (Utilities|FlowControl|Delay 0.1)
          (CallFunction|CombinationProcedure)
          (goto _label Reset))))))

(event Custom|Get%20Number%20and%20Direction
  (bind _safe_door_lock (Variables|Default|GetSafe_Door_Lock))
  (bind _relativerotation (Variables|/Script/Engine.SceneComponent|GetRelativeRotation _safe_door_lock))
  (bind _returnvalue (Class|KismetMathLibrary|ClampAxis (.roll _relativerotation)))
  (bind _returnvalue_2 (- _returnvalue 3.6e+02))
  (bind _returnvalue_3 (/ _returnvalue_2 -3.6))
  (bind _returnvalue_4 (Math|Float|Round _returnvalue_3))
  ;[1 0 0] Get Number and Direction
  (Variables|SafeCombination|SetSelected%20Direction (select (> (Variables|LockAnimation|GetDirection) 0.0) "NewEnumerator0" "NewEnumerator1"))
  (if (!= _returnvalue_4 100)
    (Variables|SafeCombination|SetSelected%20Number (Math|Conversions|ToByte(Integer) _returnvalue_4))
    (else
      (Variables|SafeCombination|SetSelected%20Number 0)))
  (Variables|/Game/InteractiveSafe/Widgets/WB_SafeNumberWidget.WB_SafeNumberWidget_C|SetSafeNumber (Variables|/Game/InteractiveSafe/Blueprint/BP_MyCharacter.BP_MyCharacter_C|GetSafeNumber%20Widget (Variables|Default|GetAs%20My%20Character)) (Utilities|Text|ToText(String) (Variables|SafeCombination|GetSelected%20Number))))

(event Custom|Add%20Selected%20Combination
  ;[1 0 0] Add To Selected Combination Or Reset
  (if (> (Utilities|Array|Length (Variables|SafeCombination|GetSafe%20Combination)) 0)
    (if (Utilities|Enum|Equal(Enum) (.Direction (Utilities|Struct|BreakST_CombinationStructure (Utilities|Array|Get(acopy) (Variables|SafeCombination|GetSafe%20Combination) (Variables|SafeCombination|GetIndex%20To%20Change)))) (Variables|SafeCombination|GetSelected%20Direction)) :!label _label
      (CallFunction|AddtoCombination (Variables|SafeCombination|GetIndex%20To%20Change))
      (elif (and (Utilities|Enum|Equal(Enum) (.Direction (Utilities|Struct|BreakST_CombinationStructure (Utilities|Array|Get(acopy) (Variables|SafeCombination|GetSafe%20Combination) (Variables|SafeCombination|GetIndex%20To%20Change)))) (.Direction (Utilities|Struct|BreakST_CombinationStructure (Utilities|Array|Get(acopy) (Variables|SafeCombination|GetSelected%20Combination) (Variables|SafeCombination|GetIndex%20To%20Change))))) (== (.Number (Utilities|Struct|BreakST_CombinationStructure (Utilities|Array|Get(acopy) (Variables|SafeCombination|GetSafe%20Combination) (Variables|SafeCombination|GetIndex%20To%20Change)))) (.Number (Utilities|Struct|BreakST_CombinationStructure (Utilities|Array|Get(acopy) (Variables|SafeCombination|GetSelected%20Combination) (Variables|SafeCombination|GetIndex%20To%20Change))))))
        (CallFunction|NextIndex)
        (goto _label)
        (else
          (Variables|SafeCombination|SetIndex%20To%20Change 0))))))

(event Custom|Check%20Combination
  ;[1 0 0] Check Combination
  (if (and (== (Utilities|Array|Length (Variables|SafeCombination|GetSafe%20Combination)) (Utilities|Array|Length (Variables|SafeCombination|GetSelected%20Combination))) (Utilities|Array|Identical (Variables|SafeCombination|GetSafe%20Combination) (Variables|SafeCombination|GetSelected%20Combination)))
    (CallFunction|HandleCorrectCombination (Variables|Settings|GetAuto%20Open?))))

(event Custom|Combination%20Procedure
  ;[1 0 0] Combination Procedure
  (CallFunction|LockSpinSound)
  (CallFunction|GetNumberandDirection)
  (CallFunction|AddSelectedCombination)
  (Utilities|FlowControl|Delay 0.05)
  (CallFunction|CheckCombination))

(event Custom|Handle%20correct%20Combination
  (params (Auto%20open? :type Boolean))
  ;[0 1 0] After correct Combination
  (Variables|Settings|SetLocked false)
  (if Auto%20open?
    (CallFunction|DeactivateUseable (Variables|Default|GetSafe_Door_Lock) "Useable")
    (CallFunction|DeactivateUseable (Variables|Default|GetSafe_Door_Handle) "Useable")
    (CallFunction|GiveInputtoPlayer)
    (CallFunction|HandleAnimation (Variables|Settings|GetLocked))
    (Utilities|FlowControl|Delay 1.6)
    (CallFunction|DoorAnimation)
    (else
      (CallFunction|DeactivateUseable (Variables|Default|GetSafe_Door_Lock) "Useable")
      (CallFunction|GiveInputtoPlayer)
      (Utilities|FlowControl|Delay 1.6))))

(event Input|EnhancedActionEvents|EnhancedInputActionIA_Back
  (params (ActionValue :type Boolean) (ElapsedSeconds :type Float%20%28double-precision%29) (TriggeredSeconds :type Float%20%28double-precision%29) (InputAction :type Input%20Action%20Object%20Reference :default "/Game/InteractiveSafe/Input/IA_Back.IA_Back"))
  ;[1 0.4452 0] INPUT Back
  (:Started
    (CallFunction|GiveInputtoPlayer)))

(event Input|EnhancedActionEvents|EnhancedInputActionIA_MoveX
  (params (ActionValue :type Float%20%28double-precision%29) (ElapsedSeconds :type Float%20%28double-precision%29) (TriggeredSeconds :type Float%20%28double-precision%29) (InputAction :type Input%20Action%20Object%20Reference :default "/Game/InteractiveSafe/Input/IA_MoveX.IA_MoveX"))
  ;[1 0.4463 0] INPUT Lock
  (:Triggered
    (CallFunction|LockRotation (- 0.0 ActionValue))))

(event EventBeginPlay
  ;[1 1 1] Cast to Player Character
  (bind _asbp_my_character (Utilities|Casting|CastToBP_MyCharacter (Game|GetPlayerCharacter 0)))
  (Variables|Default|SetAs%20My%20Character _asbp_my_character))

(event EventInteract
  (params (Component :type Actor%20Component%20Object%20Reference))
  ;[1 1 1] Check Interaction
  (if (== Component (Variables|Default|GetSafe_Door_Handle))
    (CallFunction|HandleInteracted)
    (elif (== Component (Variables|Default|GetSafe_Door_Lock))
      (CallFunction|GiveInputtoSafe))))

(fn ConstructionScript)

(fn AddtoCombination
  (params (Index :type Integer))
  (Utilities|Array|SetArrayElem (Variables|SafeCombination|GetSelected%20Combination) Index (Utilities|Struct|MakeST_CombinationStructure (Variables|SafeCombination|GetSelected%20Direction) (Variables|SafeCombination|GetSelected%20Number)) true))

(fn NextIndex
  (Variables|SafeCombination|SetIndex%20To%20Change (+ (Variables|SafeCombination|GetIndex%20To%20Change) 1))
  (return))

(fn DeactivateUseable
  (params (Component :type Actor%20Component%20Object%20Reference) (Tag%20Name :type Name))
  (bind _returnvalue (Utilities|Name|MakeLiteralName Tag%20Name))
  (bind _componenttags (Variables|/Script/Engine.ActorComponent|GetComponentTags Component))
  (bind _returnvalue_2 (Utilities|Array|FindItem _componenttags _returnvalue))
  (if (> _returnvalue_2 -1)
    (Utilities|Array|RemoveIndex (Variables|/Script/Engine.ActorComponent|GetComponentTags Component) _returnvalue_2)))