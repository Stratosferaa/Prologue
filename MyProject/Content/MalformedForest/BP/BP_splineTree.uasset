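; Procedural spline tree actor that builds a randomly winding trunk or branch in the construction script from a seeded stream, re-rolled only on Refresh.
; Random yaw steps and up/down line traces place spline points against surfaces, with optional ground-conformed ends.
; A second spline resamples the path at mesh length for spline meshes, tapered unless the end is grounded.
; Optional sphere colliders follow it, enabling randomly scattered instanced foliage.
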(fn ConstructionScript
  (bind _spline (Variables|Default|GetSpline))
  (bind _foliage_max_spawn_agle_from_top (Variables|Default|GetFoliage%20Max%20Spawn%20agle%20from%20top))
  (bind _spline_2 (Variables|Default|GetSpline))
  (bind _spline2 (Variables|Default|GetSpline2))
  (bind _random_max_rot (Variables|Default|GetRandom%20max%20rot))
  (bind _spline_3 (Variables|Default|GetSpline))
  (bind _returnvalue (Spline|GetNumberOfSplinePoints _spline))
  (bind _location (Spline|GetLocationandTangentatSplinePoint _spline_2 0 "World"))
  (bind (_x _y _z) (Math|Vector|BreakVector _location))
  (bind _returnvalue_2 (- _returnvalue 1))
  (bind (_x_2 _y_2 _z_2) (Math|Vector|BreakVector _location))
  (bind _returnvalue_3 (Spline|GetLocationatSplinePoint _spline _returnvalue_2 "World"))
  (bind (_x_3 _y_3 _z_3) (Math|Vector|BreakVector _returnvalue_3))
  (bind (_x_4 _y_4 _z_4) (Math|Vector|BreakVector _returnvalue_3))
  ;[1 1 1] When "Refresh" is clicked a new seed value for random stream is calculated. When construction scipt is otherwise updated like opening level, moving the actor etc. the seed is not recalculated and the end results stay the same.
  (if (Variables|Default|GetRefresh)
    (Variables|Default|SetSeed (Math|Random|RandomInteger 99999))
    (Variables|Default|SetRefresh false))
  ;[1 1 1] Set random seed for Stream
  (Math|Random|SetRandomStreamSeed (Variables|Default|GetRandomStream) (Variables|Default|GetSeed))
  ;[1 1 1] Set boxes location to be the location where the script starts to search the spline's first point's location.
  (Variables|Default|SetCurrent%20Start%20Loc (Transformation|GetActorLocation))
  ;[1 1 1] Points locations will be calculated using forward vector. Box's rotation is used to calculate the first forward vector.
  (Variables|Default|SetCurrentStartRot (Transformation|GetActorRotation))
  ;[1 1 1] Remove all points from spline.
  (Spline|ClearSplinePoints (Variables|Default|GetSpline) true)
  ;[1 1 1] Spline length is set by setting number of spline points. This value equals how many loops finding new locations and adding spline points to them will me calculated.
  (for _index (range 0 (- (Variables|Default|GetSplineLength%20in%20segments) 1))
    ;[1 1 1] To use later.
    (Variables|Default|SetCurrent%20index _index)
    ;[1 1 1] Randomly choose if something that we don't want to the spline to go through will be searches above or below the current start location.
    (if (Class|KismetMathLibrary|RandomBoolwithWeightfromStream (Variables|Default|GetDown-up%20weight) (Variables|Default|GetRandomStream))
      ;[1 1 1] Start linetrace from current location and end it "Max z search" length below current location.
      (bind (_outhit _returnvalue_4) (Collision|LineTraceByChannel (Variables|Default|GetCurrent%20Start%20Loc) (Math|Vector|MakeVector (.x (Variables|Default|GetCurrent%20Start%20Loc)) (.y (Variables|Default|GetCurrent%20Start%20Loc)) (- (.z (Variables|Default|GetCurrent%20Start%20Loc)) (Variables|Default|GetMax%20Z%20change))) "TraceTypeQuery1" false 0 "None" true "(R=1.000000,G=0.000000,B=0.000000,A=1.000000)" "(R=0.000000,G=1.000000,B=0.000000,A=1.000000)" 2.0))
      (if _returnvalue_4
        ;[1 1 1] If there was a hit set hit location as Current start loc.
        (Variables|Default|SetCurrent%20Start%20Loc (.Location (Collision|BreakHitResult _outhit)))
        ;[1 1 1] This variable is used at the end of this scipt. If there would be for example a landscape slope where the collision box would now be then the random location in that box could be under the landscape surface - This adjustment value is used to prevent that.
        (Variables|Default|SetAdjustmentfor%20height 125.0)
        (else
          ;[1 1 1] Linetrace did not hit anything. Set this mid-air location as the new start location.
          (Variables|Default|SetCurrent%20Start%20Loc (.TraceEnd (Collision|BreakHitResult _outhit)))))
      (else
        ;[1 1 1] Start linetrace from current location and end it "Max z search" length above current location.
        (bind (_outhit_2 _returnvalue_5) (Collision|LineTraceByChannel (Variables|Default|GetCurrent%20Start%20Loc) (Math|Vector|MakeVector (.x (Variables|Default|GetCurrent%20Start%20Loc)) (.y (Variables|Default|GetCurrent%20Start%20Loc)) (+ (.z (Variables|Default|GetCurrent%20Start%20Loc)) (Variables|Default|GetMax%20Z%20change))) "TraceTypeQuery1" false 0 "None" true "(R=1.000000,G=0.000000,B=0.000000,A=1.000000)" "(R=0.000000,G=1.000000,B=0.000000,A=1.000000)" 2.0))
        (if _returnvalue_5
          ;[1 1 1] If there was a hit set hit location as Current start loc.
          (Variables|Default|SetCurrent%20Start%20Loc (.Location (Collision|BreakHitResult _outhit_2)))
          ;[1 1 1] This variable is used at the end of this scipt. If there would be for example a ceiling of a house where the collision box would now be then the random location in that box could be aboce that ceiling - This adjustment value is used to prevent that.
          (Variables|Default|SetAdjustmentfor%20height -5e+01)
          (else
            ;[1 1 1] If there was no hit then chech if the distance between actor's location and the hit end location is not longer than "Clamp Height".
            (if (> (- (.Z (Math|Vector|BreakVector (.TraceEnd (Collision|BreakHitResult _outhit_2)))) (.Z (Math|Vector|BreakVector (Transformation|GetActorLocation)))) (Variables|Default|GetClamp%20height))
              ;[1 1 1] If the distance was greater than preferred max height then adjust the location to maximum height. The maximum height is calculated from actor's location.
              (Variables|Default|SetCurrent%20Start%20Loc (Math|Vector|MakeVector (.X (Math|Vector|BreakVector (.TraceEnd (Collision|BreakHitResult _outhit_2)))) (.Y (Math|Vector|BreakVector (.TraceEnd (Collision|BreakHitResult _outhit_2)))) (+ (.Z (Math|Vector|BreakVector (Transformation|GetActorLocation))) (Variables|Default|GetClamp%20height))))
              (else
                ;[1 1 1] Linetrace did not hit anything. Set this mid-air location as the new start location.
                (Variables|Default|SetCurrent%20Start%20Loc (.TraceEnd (Collision|BreakHitResult _outhit_2)))))))))
    ;[1 1 1] Add new spline point.
    (Spline|AddSplinePointatIndex (Variables|Default|GetSpline) (Variables|Default|GetCurrent%20Start%20Loc) (Variables|Default|GetCurrent%20index) "World" true)
    (Variables|Default|SetCurrentStartRot (Math|Rotator|MakeRotator (.Roll (Math|Rotator|BreakRotator (Variables|Default|GetCurrentStartRot))) (.Pitch (Math|Rotator|BreakRotator (Variables|Default|GetCurrentStartRot))) (+ (.Yaw (Math|Rotator|BreakRotator (Variables|Default|GetCurrentStartRot))) (Math|Random|RandomFloatinRangefromStream (* _random_max_rot -1.0) _random_max_rot (Variables|Default|GetRandomStream)))))
    ;[1 1 1] Adjustment as described earlier.
    (Variables|Default|SetCurrent%20Start%20Loc (Math|Vector|MakeVector (.X (Math|Vector|BreakVector (+ (Variables|Default|GetCurrent%20Start%20Loc) (* (Math|Vector|GetForwardVector (Math|Rotator|MakeRotator (.Roll (Math|Rotator|BreakRotator (Variables|Default|GetCurrentStartRot))) (.Pitch (Math|Rotator|BreakRotator (Variables|Default|GetCurrentStartRot))) (+ (.Yaw (Math|Rotator|BreakRotator (Variables|Default|GetCurrentStartRot))) (Math|Random|RandomFloatinRangefromStream (* _random_max_rot -1.0) _random_max_rot (Variables|Default|GetRandomStream))))) (Variables|Default|GetMax%20forward%20per%20segment))))) (.Y (Math|Vector|BreakVector (+ (Variables|Default|GetCurrent%20Start%20Loc) (* (Math|Vector|GetForwardVector (Math|Rotator|MakeRotator (.Roll (Math|Rotator|BreakRotator (Variables|Default|GetCurrentStartRot))) (.Pitch (Math|Rotator|BreakRotator (Variables|Default|GetCurrentStartRot))) (+ (.Yaw (Math|Rotator|BreakRotator (Variables|Default|GetCurrentStartRot))) (Math|Random|RandomFloatinRangefromStream (* _random_max_rot -1.0) _random_max_rot (Variables|Default|GetRandomStream))))) (Variables|Default|GetMax%20forward%20per%20segment))))) (+ (.Z (Math|Vector|BreakVector (+ (Variables|Default|GetCurrent%20Start%20Loc) (* (Math|Vector|GetForwardVector (Math|Rotator|MakeRotator (.Roll (Math|Rotator|BreakRotator (Variables|Default|GetCurrentStartRot))) (.Pitch (Math|Rotator|BreakRotator (Variables|Default|GetCurrentStartRot))) (+ (.Yaw (Math|Rotator|BreakRotator (Variables|Default|GetCurrentStartRot))) (Math|Random|RandomFloatinRangefromStream (* _random_max_rot -1.0) _random_max_rot (Variables|Default|GetRandomStream))))) (Variables|Default|GetMax%20forward%20per%20segment))))) (Variables|Default|GetAdjustmentfor%20height)))))
  (if (Variables|Default|GetConform%20end%20to%20ground)
    ;[1 1 1] Linetrace down from the location of the last spline point.
    (bind (_outhit_3 _returnvalue_6) (Collision|LineTraceByChannel (Math|Vector|MakeVector _x_3 _y_3 (- _z_3 -1e+02)) (Math|Vector|MakeVector _x_4 _y_4 (- _z_4 5e+03)) "TraceTypeQuery1" false 0 "None"))
    (if _returnvalue_6
      ;[1 1 1] Update last point location so spline will end in ground
      (Spline|SetLocationatSplinePoint (Variables|Default|GetSpline) (- (Spline|GetNumberOfSplinePoints (Variables|Default|GetSpline)) 1) (Math|Vector|MakeVector (.X (Math|Vector|BreakVector (.Location (Collision|BreakHitResult _outhit_3)))) (.Y (Math|Vector|BreakVector (.Location (Collision|BreakHitResult _outhit_3)))) (- (.Z (Math|Vector|BreakVector (.Location (Collision|BreakHitResult _outhit_3)))) (* (Variables|Default|GetMesh%20Thickness) 25.0))) "World" true)
      (else
        ;[1 1 1] If there was no hit then adjust last point location to trace end location.
        (Spline|SetLocationatSplinePoint (Variables|Default|GetSpline) (- (Spline|GetNumberOfSplinePoints (Variables|Default|GetSpline)) 1) (.TraceEnd (Collision|BreakHitResult _outhit_3)) "World" true)))
    ;[1 1 1] Linetrace down from the location of the first spline point+10 units.
    (bind (_outhit_4 _returnvalue_7) (Collision|LineTraceByChannel (Math|Vector|MakeVector _x _y (+ _z 1e+01)) (Math|Vector|MakeVector _x_2 _y_2 (- _z_2 5e+03)) "TraceTypeQuery1" false 0 "None" :!label _label))
    (if _returnvalue_7
      ;[1 1 1] Adjust first point location so spline will start from ground.
      (Spline|SetLocationatSplinePoint (Variables|Default|GetSpline) 0 (Math|Vector|MakeVector (.X (Math|Vector|BreakVector (.Location (Collision|BreakHitResult _outhit_4)))) (.Y (Math|Vector|BreakVector (.Location (Collision|BreakHitResult _outhit_4)))) (- (.Z (Math|Vector|BreakVector (.Location (Collision|BreakHitResult _outhit_4)))) (* (Variables|Default|GetMesh%20Thickness) 25.0))) "World" true)
      (else
        ;[1 1 1] If there was no hit then adjust first point location to trace end location
        (Spline|SetLocationatSplinePoint (Variables|Default|GetSpline) 0 (.TraceEnd (Collision|BreakHitResult _outhit_4)) "World" true)))
    (elif (Variables|Default|GetConform%20Start%20to%20ground)
      (goto _label)
      (else
        _)))
  ;[1 1 1] reset spline 2 points (clear).
  (Spline|ClearSplinePoints (Variables|Default|GetSpline2) true)
  ;[1 1 1] Calculating how many points spline2 is going to have.
  (for _index_2 (range 0 (.ReturnValue (Math|Float|Division(WholeandRemainder) (Spline|GetSplineLength (Variables|Default|GetSpline)) (Variables|Default|Getinput%20mesh%20lenght))))
    ;[1 1 1] Add spline2 points.
    (Spline|AddSplinePointatIndex (Variables|Default|GetSpline2) (Spline|GetLocationatDistanceAlongSpline (Variables|Default|GetSpline) (* _index_2 (Variables|Default|Getinput%20mesh%20lenght)) "Local") _index_2 "Local" true))
  ;[1 1 1] Add one more point to the end.
  (Spline|AddSplinePointatIndex _spline2 (Spline|GetLocationatSplinePoint _spline_3 (- (Spline|GetNumberOfSplinePoints _spline_3) 1) "Local") (Spline|GetNumberOfSplinePoints _spline2) "Local" true)
  ;[1 1 1] no need for spline1 points anymore, reset them (clear).
  (Spline|ClearSplinePoints (Variables|Default|GetSpline) true)
  ;[1 1 1] Calculating how many spline meshes will be added.
  (bind _output_get (Variables|Default|SetSpline2SegmentsAmount (- (Spline|GetNumberOfSplinePoints (Variables|Default|GetSpline2)) 1)))
  (for _index_3 (range 0 _output_get)
    (Variables|Default|SetCurrentSplineMeshIndex _index_3)
    (bind _returnvalue_8 (AddComponent|AddSplineMeshComponent false))
    ;[1 1 1] Set mesh
    (Variables|Default|SetCurrentSplineMesh _returnvalue_8)
    (Components|StaticMesh|SetStaticMesh (Variables|Default|GetCurrentSplineMesh) (Variables|Default|GetMesh))
    ;[1 1 1] Mesh forward axis
    (SplineMesh|SetForwardAxis (Variables|Default|GetCurrentSplineMesh) (Variables|Default|GetMesh%20forward%20Axis) true)
    ;[1 1 1] Conform end to the ground?
    (if (Variables|Default|GetConform%20end%20to%20ground)
      ;[1 1 1] Mesh scale is uniform when both ends are conformed to ground.
      (SplineMesh|SetStartScale (Variables|Default|GetCurrentSplineMesh) (* "(X=1.000000,Y=1.000000)" (Variables|Default|GetMesh%20Thickness)) true :!class /Script/Engine.SplineMeshComponent)
      (SplineMesh|SetEndScale (Variables|Default|GetCurrentSplineMesh) (* "(X=1.000000,Y=1.000000)" (Variables|Default|GetMesh%20Thickness)) true :!class /Script/Engine.SplineMeshComponent)
      (else
        ;[1 1 1] Mesh start scale is scaled down along spline distance.
        (SplineMesh|SetStartScale (Variables|Default|GetCurrentSplineMesh) (* "(X=1.000000,Y=1.000000)" (* (Variables|Default|GetMesh%20Thickness) (Variables|Default|GetCurrentEndScale))) true :!class /Script/Engine.SplineMeshComponent)
        ;[1 1 1] Mesh Scale decrement calculation.
        (Variables|Default|SetCurrentEndScale (- 1.0 (* (Variables|Default|GetCurrentSplineMeshIndex) (/ (- 1.0 0.01) (Math|Conversions|ToFloat(Integer) (Variables|Default|GetSpline2SegmentsAmount))))))
        ;[1 1 1] Mesh End scale
        (SplineMesh|SetEndScale (Variables|Default|GetCurrentSplineMesh) (* "(X=1.000000,Y=1.000000)" (* (Variables|Default|GetMesh%20Thickness) (Variables|Default|GetCurrentEndScale))) true :!class /Script/Engine.SplineMeshComponent)))
    ;[1 1 1] Conform spline meshes along spline
    (SplineMesh|SetStartandEnd (Variables|Default|GetCurrentSplineMesh) (.Location (Spline|GetLocationandTangentatSplinePoint (Variables|Default|GetSpline2) (Variables|Default|GetCurrentSplineMeshIndex) "Local")) (.Tangent (Spline|GetLocationandTangentatSplinePoint (Variables|Default|GetSpline2) (Variables|Default|GetCurrentSplineMeshIndex) "Local")) (.Location (Spline|GetLocationandTangentatSplinePoint (Variables|Default|GetSpline2) (+ (Variables|Default|GetCurrentSplineMeshIndex) 1) "Local")) (.Tangent (Spline|GetLocationandTangentatSplinePoint (Variables|Default|GetSpline2) (+ (Variables|Default|GetCurrentSplineMeshIndex) 1) "Local")) true :!class /Script/Engine.SplineMeshComponent))
  ;[1 1 1] continue adding collision meshes?
  (if (Variables|Default|GetGenerate%20collision%20meshes)
    ;[1 1 1] Amount of collision meshes based on spline lenght and mesh thickness.
    (for _index_4 (range 0 (.ReturnValue (Math|Float|Division(WholeandRemainder) (Spline|GetSplineLength (Variables|Default|GetSpline2)) (* (Variables|Default|GetMesh%20Thickness) 35.0))))
      ;[1 1 1] collision sphere scaling based on mesh thickness.
      (bind _returnvalue_9 (AddComponent|AddSphereComponent false (Math|Transform|MakeTransform "0, 0, 0" "0, 0, 0" (Math|Conversions|ToVector(Float) (* (Variables|Default|GetMesh%20Thickness) 0.7)))))
      ;[1 1 1] Collision spheres locations along spline based on mesh thickness.
      (Transformation|SetWorldLocation _returnvalue_9 (Spline|GetLocationatDistanceAlongSpline (Variables|Default|GetSpline2) (* (* _index_4 35.0) (Variables|Default|GetMesh%20Thickness)) "World") false false))
    ;[1 1 1] continue to adding foliage meshes?
    (if (Variables|Default|Getadd%20foliage%20meshes)
      ;[1 1 1] Add as many instanced mesh components as user has added foliage meshes.
      (for _index_5 (range 0 (- (Utilities|Array|Length (Variables|Default|GetFoliageMeshes)) 1))
        ;[1 1 1] Add instanced mesh component.
        (bind _returnvalue_10 (AddComponent|AddInstancedStaticMeshComponent false))
        ;[1 1 1] foliage casts shadows?
        (Rendering|SetCastShadow _returnvalue_10 (Variables|Default|GetFoliage%20Shadows?))
        ;[1 1 1] Set mesh for instanced meshes
        (Components|StaticMesh|SetStaticMesh _returnvalue_10 (Utilities|Array|Get(acopy) (Variables|Default|GetFoliageMeshes) _index_5))
        ;[1 1 1] Add instanced mesh to array
        (Utilities|Array|Add (Variables|Default|GetInstancedMeshes) _returnvalue_10))
      ;[1 1 1] how many foliage mesh instances?
      (for _index_6 (range 0 (- (Variables|Default|Getfoliage%20amount) 1))
        ;[1 1 1] Random distance along spline to variable.
        (Variables|Default|SetCurrentDistance (Math|Random|RandomFloatinRangefromStream 0.0 (Spline|GetSplineLength (Variables|Default|GetSpline2)) (Variables|Default|GetRandomStream)))
        ;[1 1 1] Current random instanced mesh component to variable.
        (bind _output_get_2 (Variables|Default|SetCurrentSelectInt (Math|Integer|SelectInt 0 (Math|Random|RandomIntegerinRangefromStream 1 (- (Utilities|Array|Length (Variables|Default|GetInstancedMeshes)) 1) (Variables|Default|GetRandomStream)) (Class|KismetMathLibrary|RandomBoolwithWeightfromStream (* (Variables|Default|GetFoliage%20element%200%20bias%20multiplier) 0.03) (Variables|Default|GetRandomStream)))))
        ;[1 1 1] If foliage mesh index 0 is selected set "Pick A" to TRUE so it's size scalar can be modified seperately.
        (if (== _output_get_2 0)
          (Variables|Default|SetPick%20A true)
          (else
            (Variables|Default|SetPick%20A false)))
        ;[1 1 1] Current instanced mesh variable.
        (Variables|Default|SetCurrentInstancedMesh (Utilities|Array|Get(acopy) (Variables|Default|GetInstancedMeshes) (Variables|Default|GetCurrentSelectInt)))
        ;[1 1 1] Add foliage mesh instance.
        (Components|InstancedStaticMesh|AddInstance (Variables|Default|GetCurrentInstancedMesh) (Math|Transform|MakeTransform (+ (* (Math|Vector|GetUpVector (Math|Rotator|MakeRotator (Math|Random|RandomFloatinRangefromStream (* _foliage_max_spawn_agle_from_top -1.0) _foliage_max_spawn_agle_from_top (Variables|Default|GetRandomStream)) (.Pitch (Math|Rotator|BreakRotator (Spline|GetRotationatDistanceAlongSpline (Variables|Default|GetSpline2) (Variables|Default|GetCurrentDistance) "World"))) (.Yaw (Math|Rotator|BreakRotator (Spline|GetRotationatDistanceAlongSpline (Variables|Default|GetSpline2) (Variables|Default|GetCurrentDistance) "World"))))) (* (Variables|Default|GetMesh%20Thickness) (Variables|Default|GetFoliage%20local%20Z%20offset))) (Spline|GetLocationatDistanceAlongSpline (Variables|Default|GetSpline2) (Variables|Default|GetCurrentDistance) "Local")) (Math|Rotator|MakeRotator (Math|Random|RandomFloatinRangefromStream (* _foliage_max_spawn_agle_from_top -1.0) _foliage_max_spawn_agle_from_top (Variables|Default|GetRandomStream)) (.Pitch (Math|Rotator|BreakRotator (Spline|GetRotationatDistanceAlongSpline (Variables|Default|GetSpline2) (Variables|Default|GetCurrentDistance) "World"))) (.Yaw (Math|Rotator|BreakRotator (Spline|GetRotationatDistanceAlongSpline (Variables|Default|GetSpline2) (Variables|Default|GetCurrentDistance) "World")))) (Math|Conversions|ToVector(Float) (Math|Float|SelectFloat (* (Variables|Default|GetFoliage%20Element%200%20Scaler) (Math|Random|RandomFloatinRangefromStream 0.7 1.8 (Variables|Default|GetRandomStream))) (* (Math|Random|RandomFloatinRangefromStream 0.7 1.8 (Variables|Default|GetRandomStream)) (Variables|Default|GetFoliage%20scaler)) (Variables|Default|GetPick%20A)))))
        ;[1 1 1] Foliage mesh collision on/off?
        (if (not (Variables|Default|GetFoliage%20mesh%20has%20collision?))
          (Collision|SetCollisionEnabled (Variables|Default|GetCurrentInstancedMesh) "NoCollision"))))))