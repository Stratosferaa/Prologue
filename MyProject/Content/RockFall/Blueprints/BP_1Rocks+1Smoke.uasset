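; Rock fall effect actor that drives a one-rock, one-smoke Niagara system with optional repeatable, attenuated sound.
; PlaySequence pushes the Rock1MiniGravel settings struct into the Niagara system as prefixed variables and plays the rock sound, using a DoOnce that resets after one second to limit retriggering.
; The construction script sets up the editor-visible sound attenuation range, applies the same Niagara variables, then calls PlaySequence.
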(event Custom|PlaySequence
  (bind _soundattenuationrange (Variables|SOUNDPARAMETERS:|GetSoundAttenuationRange))
  (Utilities|FlowControl|DoOnce false :!label _label
    (:Completed
      (Utilities|FlowControl|Sequence
        (:then_0
          ;[1 1 1] Emitter 1: At 0 second:
          ; Mini Rocks(Stones)Start
          (CallFunction|NiagaraSystemVariable (Variables|Default|GetNS_AMCF-1Rock+1Smoke) (Variables|ROCKSPARAMETERS:|GetRock1:MiniGravel) 1)
          ;[1 1 1] Sound
          (Utilities|PlayRockSound (Variables|SOUNDPARAMETERS:|GetSoundActive) (Variables|SOUNDPARAMETERS:|GetSound) (Variables|SOUNDPARAMETERS:|GetVolume) (Variables|SOUNDPARAMETERS:|GetRepeatPlaySound) (Variables|SOUNDPARAMETERS:|GetDelayBeforeRepeatSound) (Variables|SOUNDPARAMETERS:|GetSoundAttenuation) (.x _soundattenuationrange) (.y _soundattenuationrange) 0.0 (Variables|Default|GetAttenuation1)))
        (:then_1
          (Utilities|FlowControl|Delay 1.0)
          (goto _label Reset))))))

(fn ConstructionScript
  (CallFunction|EmitterAttenuation (Variables|Default|GetSphereInnerRadius) (Variables|Default|GetSphereFallOff) (Variables|SOUNDPARAMETERS:|GetSoundAttenuationEditorVisibility) (Variables|SOUNDPARAMETERS:|GetSoundAttenuationRange))
  ;[1 1 1] Emitter 1: At 0 second:
  ; Mini Rocks(Stones)Start
  (CallFunction|NiagaraSystemVariable (Variables|Default|GetNS_AMCF-1Rock+1Smoke) (Variables|ROCKSPARAMETERS:|GetRock1:MiniGravel) 1)
  (CallFunction|PlaySequence))