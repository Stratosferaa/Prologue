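; Rock fall effect Blueprint that plays a two-emitter gravel Niagara system (2 rocks, 2 smoke) with two configurable sounds.
; PlaySequence activates the system, pushes each emitter's settings struct into prefixed Niagara variables, and plays both sounds with optional repeat and attenuation.
; A DoOnce gate resets after a one-second delay.
; The construction script updates attenuation spheres, applies the same Niagara variables and calls PlaySequence for editor preview.
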(event Custom|PlaySequence
  (bind _2_soundattenuationrange (Variables|SOUND2PARAMETERS:|Get2-SoundAttenuationRange))
  (bind _ns_amcf_2rocks_2smoke (Variables|Default|GetNS_AMCF-2Rocks+2Smoke))
  (bind _1_soundattenuationrange (Variables|SOUND1PARAMETERS:|Get1-SoundAttenuationRange))
  (Utilities|FlowControl|DoOnce false :!label _label
    (:Completed
      (Components|Activation|Activate (Variables|Default|GetNS_AMCF-2Rocks+2Smoke) false)
      (Utilities|FlowControl|Sequence
        (:then_0
          ;[1 1 1] Emitter 1: At 0 second:
          ; Mini Rocks(Stones)Start
          (CallFunction|NiagaraSystemVariable _ns_amcf_2rocks_2smoke (Variables|ROCKSPARAMETERS:|GetRock1:MiniGravel) 1)
          ;[1 1 1] Emitter 2: At 3 seconds:
          ; Small Rock Start
          (CallFunction|NiagaraSystemVariable _ns_amcf_2rocks_2smoke (Variables|ROCKSPARAMETERS:|GetRock2:SmallGravel) 2))
        (:then_1
          ;[1 1 1] Sound 1
          (Utilities|PlayRockSound (Variables|SOUND1PARAMETERS:|Get1-SoundActive) (Variables|SOUND1PARAMETERS:|Get1-Sound) (Variables|SOUND1PARAMETERS:|Get1-Volume) (Variables|SOUND1PARAMETERS:|Get1-RepeatPlaySound) (Variables|SOUND1PARAMETERS:|Get1-DelayBeforeRepeatSound) (Variables|SOUND1PARAMETERS:|Get1-SoundAttenuation) (.x _1_soundattenuationrange) (.y _1_soundattenuationrange) (Variables|SOUND1PARAMETERS:|Get1-DelayToStartSOUND_2) (Variables|Default|GetAttenuation1))
          ;[1 1 1] Sound 2
          (Utilities|PlayRockSound (Variables|SOUND2PARAMETERS:|Get2-SoundActive) (Variables|SOUND2PARAMETERS:|Get2-Sound) (Variables|SOUND2PARAMETERS:|Get2-Volume) (Variables|SOUND2PARAMETERS:|Get2-RepeatPlaySound) (Variables|SOUND2PARAMETERS:|Get2-DelayBeforeRepeatSound) (Variables|SOUND2PARAMETERS:|Get2-SoundAttenuation) (.x _2_soundattenuationrange) (.y _2_soundattenuationrange) 0.0 (Variables|Default|GetAttenuation2)))
        (:then_2
          (Utilities|FlowControl|Delay 1.0)
          (goto _label Reset))))))

(fn ConstructionScript
  (bind _ns_amcf_2rocks_2smoke (Variables|Default|GetNS_AMCF-2Rocks+2Smoke))
  (CallFunction|EmitterAttenuation (Variables|Default|Get1-SphereInnerRadius) (Variables|Default|Get1-SphereFallOff) (Variables|SOUND1PARAMETERS:|Get1-SoundAttenuationEditorVisibility) (Variables|SOUND1PARAMETERS:|Get1-SoundAttenuationRange))
  (CallFunction|EmitterAttenuation (Variables|Default|Get2-SphereInnerRadius) (Variables|Default|Get2-SphereFallOff) (Variables|SOUND2PARAMETERS:|Get2-SoundAttenuationEditorVisibility) (Variables|SOUND2PARAMETERS:|Get2-SoundAttenuationRange))
  ;[1 1 1] Emitter 1: At 0 second:
  ; Mini Rocks(Stones)Start
  (CallFunction|NiagaraSystemVariable _ns_amcf_2rocks_2smoke (Variables|ROCKSPARAMETERS:|GetRock1:MiniGravel) 1)
  ;[1 1 1] Emitter 2: At 3 seconds:
  ; Small Rock Start
  (CallFunction|NiagaraSystemVariable _ns_amcf_2rocks_2smoke (Variables|ROCKSPARAMETERS:|GetRock2:SmallGravel) 2)
  (CallFunction|PlaySequence))