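; Rockfall effect actor that plays a Niagara system of rocks and smoke with four layered sounds.
; PlaySequence activates the system, pushes four rock-size variable structs into prefixed emitters, and runs configurable, staggered sounds with optional repeats and attenuation.
; A DoOnce that resets after one second limits retriggering.
; The construction script updates attenuation range spheres, applies the same Niagara variables and calls PlaySequence.
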(event Custom|PlaySequence
  (bind _ns_amcf_4rocks_4smoke (Variables|Default|GetNS_AMCF-4Rocks+4Smoke))
  (bind _2_soundattenuationrange (Variables|SOUND2PARAMETERS:|Get2-SoundAttenuationRange))
  (bind _3_soundattenuationrange (Variables|SOUND3PARAMETERS:|Get3-SoundAttenuationRange))
  (bind _4_soundattenuationrange (Variables|SOUND4PARAMETERS:|Get4-SoundAttenuationRange))
  (bind _1_soundattenuationrange (Variables|SOUND1PARAMETERS:|Get1-SoundAttenuationRange))
  (Utilities|FlowControl|DoOnce false :!label _label
    (:Completed
      (Components|Activation|Activate (Variables|Default|GetNS_AMCF-4Rocks+4Smoke) false)
      (Utilities|FlowControl|Sequence
        (:then_0
          ;[1 1 1] Emitter 1: At 0 second:
          ; Gravel Start
          (CallFunction|NiagaraSystemVariable _ns_amcf_4rocks_4smoke (Variables|ROCKSPARAMETERS:|GetRock1:MiniGravel) 1)
          ;[1 1 1] Emitter 2: At 2 seconds:
          ; Mini Rocks(Stones)Start
          (CallFunction|NiagaraSystemVariable _ns_amcf_4rocks_4smoke (Variables|ROCKSPARAMETERS:|GetRock2:SmallGravel) 2)
          ;[1 1 1] Emitter 3: At 3 seconds:
          ; Small Rock Start
          (CallFunction|NiagaraSystemVariable _ns_amcf_4rocks_4smoke (Variables|ROCKSPARAMETERS:|GetRock3:Gravel) 3)
          ;[1 1 1] Emitter 4: At 4 second:
          ; Medium Rock Start
          (CallFunction|NiagaraSystemVariable _ns_amcf_4rocks_4smoke (Variables|ROCKSPARAMETERS:|GetRock4:Medium) 4))
        (:then_1
          ;[1 1 1] Sound 1
          (Utilities|PlayRockSound (Variables|SOUND1PARAMETERS:|Get1-SoundActive) (Variables|SOUND1PARAMETERS:|Get1-Sound) (Variables|SOUND1PARAMETERS:|Get1-Volume) (Variables|SOUND1PARAMETERS:|Get1-RepeatPlaySound) (Variables|SOUND1PARAMETERS:|Get1-DelayBeforeRepeatSound) (Variables|SOUND1PARAMETERS:|Get1-SoundAttenuation) (.x _1_soundattenuationrange) (.y _1_soundattenuationrange) (Variables|SOUND1PARAMETERS:|Get1-DelayToStartSOUND_2) (Variables|Default|GetAttenuation1))
          ;[1 1 1] Sound 2
          (Utilities|PlayRockSound (Variables|SOUND2PARAMETERS:|Get2-SoundActive) (Variables|SOUND2PARAMETERS:|Get2-Sound) (Variables|SOUND2PARAMETERS:|Get2-Volume) (Variables|SOUND2PARAMETERS:|Get2-RepeatPlaySound) (Variables|SOUND2PARAMETERS:|Get2-DelayBeforeRepeatSound) (Variables|SOUND2PARAMETERS:|Get2-SoundAttenuation) (.x _2_soundattenuationrange) (.y _2_soundattenuationrange) (Variables|SOUND2PARAMETERS:|Get2-DelayToStartSOUND_3) (Variables|Default|GetAttenuation2))
          ;[1 1 1] Sound 3
          (Utilities|PlayRockSound (Variables|SOUND3PARAMETERS:|Get3-SoundActive) (Variables|SOUND3PARAMETERS:|Get3-Sound) (Variables|SOUND3PARAMETERS:|Get3-Volume) (Variables|SOUND3PARAMETERS:|Get3-RepeatPlaySound) (Variables|SOUND3PARAMETERS:|Get3-DelayBeforeRepeatSound) (Variables|SOUND3PARAMETERS:|Get3-SoundAttenuation) (.x _3_soundattenuationrange) (.y _3_soundattenuationrange) (Variables|SOUND3PARAMETERS:|Get3-DelayToStartSOUND_4) (Variables|Default|GetAttenuation3))
          ;[1 1 1] Sound 4
          (Utilities|PlayRockSound (Variables|SOUND4PARAMETERS:|Get4-SoundActive) (Variables|SOUND4PARAMETERS:|Get4-Sound) (Variables|SOUND4PARAMETERS:|Get4-Volume) (Variables|SOUND4PARAMETERS:|Get4-RepeatPlaySound) (Variables|SOUND4PARAMETERS:|Get4-DelayBeforeRepeatSound) (Variables|SOUND4PARAMETERS:|Get4-SoundAttenuation) (.x _4_soundattenuationrange) (.y _4_soundattenuationrange) 0.0 (Variables|Default|GetAttenuation4)))
        (:then_2
          (Utilities|FlowControl|Delay 1.0)
          (goto _label Reset))))))

(fn ConstructionScript
  (bind _ns_amcf_4rocks_4smoke (Variables|Default|GetNS_AMCF-4Rocks+4Smoke))
  (CallFunction|EmitterAttenuation (Variables|Default|Get1-SphereInnerRadius) (Variables|Default|Get1-SphereFallOff) (Variables|SOUND1PARAMETERS:|Get1-SoundAttenuationEditorVisibility) (Variables|SOUND1PARAMETERS:|Get1-SoundAttenuationRange))
  (CallFunction|EmitterAttenuation (Variables|Default|Get2-SphereInnerRadius) (Variables|Default|Get2-SphereFallOff) (Variables|SOUND2PARAMETERS:|Get2-SoundAttenuationEditorVisibility) (Variables|SOUND2PARAMETERS:|Get2-SoundAttenuationRange))
  (CallFunction|EmitterAttenuation (Variables|Default|Get3-SphereInnerRadius) (Variables|Default|Get3-SphereFallOff) (Variables|SOUND3PARAMETERS:|Get3-SoundAttenuationEditorVisibility) (Variables|SOUND3PARAMETERS:|Get3-SoundAttenuationRange))
  (CallFunction|EmitterAttenuation (Variables|Default|Get4-SphereInnerRadius) (Variables|Default|Get4-SphereFallOff) (Variables|SOUND4PARAMETERS:|Get4-SoundAttenuationEditorVisibility) (Variables|SOUND4PARAMETERS:|Get4-SoundAttenuationRange))
  ;[1 1 1] Emitter 1: At 0 second:
  ; Gravel Start
  (CallFunction|NiagaraSystemVariable _ns_amcf_4rocks_4smoke (Variables|ROCKSPARAMETERS:|GetRock1:MiniGravel) 1)
  ;[1 1 1] Emitter 2: At 2 seconds:
  ; Mini Rocks(Stones)Start
  (CallFunction|NiagaraSystemVariable _ns_amcf_4rocks_4smoke (Variables|ROCKSPARAMETERS:|GetRock2:SmallGravel) 2)
  ;[1 1 1] Emitter 3: At 3 seconds:
  ; Small Rock Start
  (CallFunction|NiagaraSystemVariable _ns_amcf_4rocks_4smoke (Variables|ROCKSPARAMETERS:|GetRock3:Gravel) 3)
  ;[1 1 1] Emitter 4: At 4 second:
  ; Medium Rock Start
  (CallFunction|NiagaraSystemVariable _ns_amcf_4rocks_4smoke (Variables|ROCKSPARAMETERS:|GetRock4:Medium) 4)
  (CallFunction|PlaySequence))