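; Scene capture actor for interactive foliage that records tagged force objects around the player.
; On BeginPlay it writes the capture's ortho width to a material parameter collection and sets primitives tagged InteractiveForce, on actors with that tag, as show-only components.
; Each tick it follows the player character in X and Y at a fixed height and publishes its location to the same collection as CaptureLocation.
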(event EventBeginPlay
  (CallFunction|SetCaptureSize)
  (bind _outactors (Actor|GetAllActorswithTag "InteractiveForce"))
  (for _array_element _outactors
    (for _array_element_2 (Actor|GetComponentsbyTag _array_element "/Script/Engine.PrimitiveComponent" "InteractiveForce")
      (Rendering|SceneCapture|ShowOnlyComponent (Variables|Default|GetInteractiveFoliageCapture) _array_element_2))))

(event EventTick
  (params (DeltaSeconds :type Float%20%28single-precision%29))
  (CallFunction|MoveCapture))

(fn ConstructionScript)

(fn MoveCapture
  (bind _returnvalue (Game|GetPlayerCharacter 0))
  (bind _returnvalue_2 (Transformation|GetActorLocation _returnvalue))
  (Transformation|SetActorLocation (Math|Vector|MakeVector (.x _returnvalue_2) (.y _returnvalue_2) (.z (Transformation|GetActorLocation))) false false)
  (Rendering|Material|SetVectorParameterValue "/Game/RuinedCrypt/Effects/InteractiveFoliage_01/mpc_InteractiveFoliage_01_01.mpc_InteractiveFoliage_01_01" "CaptureLocation" (Math|Conversions|ToLinearColor(Vector) (Transformation|GetActorLocation)) :!class /Script/Engine.KismetMaterialLibrary))

(fn SetCaptureSize
  (Rendering|Material|SetScalarParameterValue "/Game/RuinedCrypt/Effects/InteractiveFoliage_01/mpc_InteractiveFoliage_01_01.mpc_InteractiveFoliage_01_01" "CaptureSize" (Variables|/Script/Engine.SceneCaptureComponent2D|GetOrthoWidth (Variables|Default|GetInteractiveFoliageCapture)) :!class /Script/Engine.KismetMaterialLibrary))