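; Rat effect actor that sends a rat particle scurrying between holes along its splines, with a squeak sound while it runs.
; Construction gathers spline components; at play a timeline moves the rat along a random spline at random speed, hides it, then repeats after a random delay.
; Optional depth correction briefly captures tagged meshes into an orthographic depth render target, then feeds it to the rat's dynamic material.
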(event EventBeginPlay
  (bind _scenecapturecomponent2d (Variables|Default|GetSceneCaptureComponent2D))
  (bind _splinesarray (Variables|Default|GetSplinesArray))
  (bind _scenecapturecomponent2d_2 (Variables|Default|GetSceneCaptureComponent2D))
  (bind _returnvalue (Utilities|Array|Length _splinesarray))
  (Utilities|FlowControl|Sequence
    (:then_0
      ;[1 1 1] Init Depth Correction
      (if (Variables|Default|GetUseDepthCorrection)
        (Utilities|IsValid (Variables|Default|GetRatsMaterial)
          (:Is%20Valid
            (bind _returnvalue_2 (Rendering|CreateRenderTarget2D 128 128 "RTF_R16f"))
            (Variables|Default|SetRT_Texture _returnvalue_2)
            (Variables|/Script/Engine.SceneCaptureComponent2D|SetTextureTarget _scenecapturecomponent2d_2 (Variables|Default|GetRT_Texture))
            (bind _outactors (Actor|GetAllActorswithTag (Variables|Default|GetMeshTag)))
            (Variables|/Script/Engine.SceneCaptureComponent|SetShowOnlyActors _scenecapturecomponent2d_2 _outactors)
            (Variables|/Script/Engine.SceneCaptureComponent|SetbCaptureEveryFrame _scenecapturecomponent2d_2 true)
            (Utilities|FlowControl|Delay 0.1)
            (Variables|/Script/Engine.SceneCaptureComponent|SetbCaptureEveryFrame _scenecapturecomponent2d_2 false)
            (bind _returnvalue_3 (Rendering|Material|CreateDynamicMaterialInstance (Variables|Default|GetRatsMaterial) "None" :!class /Script/Engine.KismetMaterialLibrary))
            (Variables|Default|SetMID _returnvalue_3)
            (Rendering|Material|SetTextureParameterValue (Variables|Default|GetMID) "DepthTexture" (Variables|Default|GetRT_Texture))
            (Rendering|Material|SetScalarParameterValue (Variables|Default|GetMID) "DepthOrtho" (Variables|/Script/Engine.SceneCaptureComponent2D|GetOrthoWidth _scenecapturecomponent2d) :!class /Script/Engine.MaterialInstanceDynamic)
            (Rendering|Material|SetVectorParameterValue (Variables|Default|GetMID) "DepthPosition" (Math|Conversions|ToLinearColor(Vector) (Transformation|GetWorldLocation _scenecapturecomponent2d)) :!class /Script/Engine.MaterialInstanceDynamic)
            (Rendering|Material|SetMaterial (Variables|Default|GetRatParticle) 0 (Variables|Default|GetMID))))))
    (:then_1
      ;[1 1 1] Rat Animation
      (if (> _returnvalue 0)
        (Development|SetHiddeninGame (Variables|Default|GetRatParticle) false false :!label _label)
        (Variables|Default|SetSplineComponent (Utilities|Array|Get(acopy) _splinesarray (Math|Random|RandomInteger _returnvalue)))
        (Components|Timeline|SetPlayRate (Variables|Default|GetSplineAnimation) (/ 1.0 (Math|Random|RandomFloatinRange (Variables|Default|GetRatSpeedMin) (Variables|Default|GetRatSpeedMax))))
        (Utilities|FlowControl|Sequence
          (:then_0
            (bind _time (Timeline|SplineAnimation PlayFromStart)
              (:Update
                (Transformation|SetWorldLocationAndRotation (Variables|Default|GetRatParticle) (Spline|GetLocationatDistanceAlongSpline (Variables|Default|GetSplineComponent) (Math|Float|Lerp 0.0 (Spline|GetSplineLength (Variables|Default|GetSplineComponent)) _time) "World") (Spline|GetRotationatDistanceAlongSpline (Variables|Default|GetSplineComponent) (Math|Float|Lerp 0.0 (Spline|GetSplineLength (Variables|Default|GetSplineComponent)) _time) "World") false false))
              (:Finished
                (Development|SetHiddeninGame (Variables|Default|GetRatParticle) true false)
                (Utilities|FlowControl|Sequence
                  (:then_0
                    (Utilities|FlowControl|Delay (Math|Random|RandomFloatinRange (Variables|Default|GetDelayMin) (Variables|Default|GetDelayMax)))
                    (goto _label))
                  (:then_1
                    (Audio|Components|Audio|Stop (Variables|Default|GetS_RatSqueak_01_01_Cue)))))))
          (:then_1
            (Audio|Components|Audio|Play (Variables|Default|GetS_RatSqueak_01_01_Cue) 0.0)))))))

(event Collision|EventActorBeginOverlap
  (params (OtherActor :type Actor%20Object%20Reference)))

(event EventTick
  (params (DeltaSeconds :type Float%20%28single-precision%29)))

(fn ConstructionScript
  (Variables|Default|SetSplinesArray (Actor|GetComponentsByClass "/Script/Engine.SplineComponent")))