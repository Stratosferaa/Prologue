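; Rat swarm effect actor that feeds a one-time depth capture of tagged meshes into the rat particle material for depth correction.
; On BeginPlay a SceneCapture2D renders only actors with MeshTag into a small R16f render target, then stops capturing after a brief delay.
; A dynamic material receives that texture, ortho width and capture position, then replaces the particle system's material.
; The squeak sound overlap logic is disconnected.
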(event OnComponentBeginOverlap(Squeak_Sound_Collision_Sphere)
  (params (OverlappedComponent :type Primitive%20Component%20Object%20Reference) (OtherActor :type Actor%20Object%20Reference) (OtherComp :type Primitive%20Component%20Object%20Reference) (OtherBodyIndex :type Integer) (bFromSweep :type Boolean) (SweepResult :type Hit%20Result%20Structure%20%28by%20ref%29))
  ;[1 0 0.02983] Squeaking sounds logic ## trzeba fixnąć i zrobić tak jak Michałowi przekazywałem
)

(event OnComponentEndOverlap(Squeak_Sound_Collision_Sphere)
  (params (OverlappedComponent :type Primitive%20Component%20Object%20Reference) (OtherActor :type Actor%20Object%20Reference) (OtherComp :type Primitive%20Component%20Object%20Reference) (OtherBodyIndex :type Integer))
  ;[1 0 0.02983] Squeaking sounds logic ## trzeba fixnąć i zrobić tak jak Michałowi przekazywałem
)

(event EventBeginPlay
  (bind _scenecapturecomponent2d (Variables|Default|GetSceneCaptureComponent2D))
  (bind _scenecapturecomponent2d_2 (Variables|Default|GetSceneCaptureComponent2D))
  (Utilities|IsValid (Variables|Default|GetRatsParticle)
    (:Is%20Valid
      (Utilities|IsValid (Variables|Default|GetRatsMaterial)
        (:Is%20Valid
          (bind _returnvalue (Rendering|CreateRenderTarget2D 128 128 "RTF_R16f"))
          (Variables|Default|SetRT_Texture _returnvalue)
          (Variables|/Script/Engine.SceneCaptureComponent2D|SetTextureTarget _scenecapturecomponent2d (Variables|Default|GetRT_Texture))
          (bind _outactors (Actor|GetAllActorswithTag (Variables|Default|GetMeshTag)))
          (Variables|/Script/Engine.SceneCaptureComponent|SetShowOnlyActors _scenecapturecomponent2d _outactors)
          (Variables|/Script/Engine.SceneCaptureComponent|SetbCaptureEveryFrame _scenecapturecomponent2d true)
          (Utilities|FlowControl|Delay 0.1)
          (Variables|/Script/Engine.SceneCaptureComponent|SetbCaptureEveryFrame _scenecapturecomponent2d false)
          (bind _returnvalue_2 (Rendering|Material|CreateDynamicMaterialInstance (Variables|Default|GetRatsMaterial) "None" :!class /Script/Engine.KismetMaterialLibrary))
          (Variables|Default|SetMID _returnvalue_2)
          (Rendering|Material|SetTextureParameterValue (Variables|Default|GetMID) "DepthTexture" (Variables|Default|GetRT_Texture))
          (Rendering|Material|SetScalarParameterValue (Variables|Default|GetMID) "DepthOrtho" (Variables|/Script/Engine.SceneCaptureComponent2D|GetOrthoWidth _scenecapturecomponent2d_2) :!class /Script/Engine.MaterialInstanceDynamic)
          (Rendering|Material|SetVectorParameterValue (Variables|Default|GetMID) "DepthPosition" (Math|Conversions|ToLinearColor(Vector) (Transformation|GetWorldLocation _scenecapturecomponent2d_2)) :!class /Script/Engine.MaterialInstanceDynamic)
          (Rendering|Material|SetMaterial (Variables|/Script/Engine.Emitter|GetParticleSystemComponent (Variables|Default|GetRatsParticle)) 0 (Variables|Default|GetMID)))))))

(event Collision|EventActorBeginOverlap
  (params (OtherActor :type Actor%20Object%20Reference)))

(event EventTick
  (params (DeltaSeconds :type Float%20%28single-precision%29)))

(fn ConstructionScript)