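; Quest manager that tracks completion of item-based quests configured in the НастройкаКвестов array and reports it to the W_Quest widget.
; Qestupdatestat finds the first quest containing the given item, checks its type, and marks the item or single-item quest complete.
; It then refreshes the widget with the whole array.
; Setup logic for creating the widget, sizing completion flags and linking items back is disconnected, and BeginPlay is empty.
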(event Custom|Qest%20update%20stat
  (params (Item :type BP%20Base%20Item%20Object%20Reference) (Enum_QestTupe :type Enum_QestTupe%20Enum :default "NewEnumerator0"))
  (bind _настройка_квестов (Variables|Default|GetНастройка%20квестов))
  (Variables|Default|SetArray%20Index -1)
  (bind (_array_element _array_index) (Utilities|Array|ForEachLoopwithBreak _настройка_квестов :!label _label)
    (:LoopBody
      (if (not (== (Utilities|Array|FindItem (.Итемы (Utilities|Struct|Breakstr_qest _array_element)) Item) -1))
        (Variables|Default|SetArray%20Index _array_index)
        (goto _label Break)))
    (:Completed
      (if (not (== (Variables|Default|GetArray%20Index) -1))
        (if (Utilities|Enum|Equal(Enum) (.Типквеста (Utilities|Struct|Breakstr_qest (Utilities|Array|Get(acopy) _настройка_квестов (Variables|Default|GetArray%20Index)))) Enum_QestTupe)
          (if (== (Utilities|Array|Length (.Итемы (Utilities|Struct|Breakstr_qest (Utilities|Array|Get(acopy) _настройка_квестов (Variables|Default|GetArray%20Index))))) 1)
            (|SetBy-RefVar (Utilities|Array|Get(acopy) _настройка_квестов (Variables|Default|GetArray%20Index)) (Utilities|Struct|Makestr_qest (.описаниеквеста (Utilities|Struct|Breakstr_qest (Utilities|Array|Get(acopy) _настройка_квестов (Variables|Default|GetArray%20Index)))) (.Типквеста (Utilities|Struct|Breakstr_qest (Utilities|Array|Get(acopy) _настройка_квестов (Variables|Default|GetArray%20Index)))) (.Итемы (Utilities|Struct|Breakstr_qest (Utilities|Array|Get(acopy) _настройка_квестов (Variables|Default|GetArray%20Index)))) (.Complited (Utilities|Struct|Breakstr_qest (Utilities|Array|Get(acopy) _настройка_квестов (Variables|Default|GetArray%20Index)))) true))
            (Default|UpdateStatQests (Variables|Default|GetW_Quest) (Variables|Default|GetНастройка%20квестов))
            (else
              (bind _output_get (Variables|Default|SetComplited (.Complited (Utilities|Struct|Breakstr_qest (Utilities|Array|Get(acopy) _настройка_квестов (Variables|Default|GetArray%20Index))))))
              (Utilities|Array|SetArrayElem _output_get (Utilities|Array|FindItem (.Итемы (Utilities|Struct|Breakstr_qest (Utilities|Array|Get(acopy) _настройка_квестов (Variables|Default|GetArray%20Index)))) Item) true)
              (|SetBy-RefVar (Utilities|Array|Get(acopy) _настройка_квестов (Variables|Default|GetArray%20Index)) (Utilities|Struct|Makestr_qest (.описаниеквеста (Utilities|Struct|Breakstr_qest (Utilities|Array|Get(acopy) _настройка_квестов (Variables|Default|GetArray%20Index)))) (.Типквеста (Utilities|Struct|Breakstr_qest (Utilities|Array|Get(acopy) _настройка_квестов (Variables|Default|GetArray%20Index)))) (.Итемы (Utilities|Struct|Breakstr_qest (Utilities|Array|Get(acopy) _настройка_квестов (Variables|Default|GetArray%20Index)))) (Variables|Default|GetComplited) (== (Utilities|Array|FindItem (Variables|Default|GetComplited) false) -1)))
              (Default|UpdateStatQests (Variables|Default|GetW_Quest) (Variables|Default|GetНастройка%20квестов)))))))))

(event EventBeginPlay)

(fn ConstructionScript)