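; Construction-script Blueprint that grows a procedural vine of spline meshes along surrounding surfaces.
; Each segment line-traces forward, or down on a miss, then moves the arrow to the result and orients it by the normal plus seeded random noise, adding a spline point.
; A second spline resamples that path at mesh-length intervals and carries the spline mesh components, with both ends scaled to zero for tapered tips.
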(event EventBeginPlay)

(event Collision|EventActorBeginOverlap
  (params (OtherActor :type Actor%20Object%20Reference)))

(event EventTick
  (params (DeltaSeconds :type Float%20%28single-precision%29)))

(fn ConstructionScript
  (bind _scale (Variables|Default|GetScale))
  (bind _noise (Variables|Default|GetNoise))
  (bind _mesh (Variables|Default|GetMesh))
  (bind _arrow (Variables|Default|GetArrow))
  (bind _returnvalue (* "(X=1.000000,Y=1.000000)" _scale))
  ;[1 1 1] Stream seed
  (if (Variables|Default|GetNewSeed)
    (Variables|Default|SetSeed (Math|Random|RandomIntegerinRange 0 9999))
    (Variables|Default|SetNewSeed false))
  (Math|Random|SetRandomStreamSeed (Variables|Default|GetStream) (Variables|Default|GetSeed))
  ;[1 1 1] Remove Spline points from spline #1
  (Spline|ClearSplinePoints (Variables|Default|GetSpline) true)
  ;[1 1 1] Set parameters from arrow transform
  (Variables|Default|SetUpvector (Math|Vector|GetUpVector _arrow))
  (Variables|Default|SetForwardVector (Math|Vector|GetForwardVector _arrow))
  (Variables|Default|SetRightVector (Math|Vector|GetRightVector _arrow))
  (Variables|Default|SetLocation (Transformation|GetWorldLocation _arrow))
  ;[1 1 1] How many segments to process?
  (for _index (range 0 (Variables|Default|GetSegments))
    ;[1 1 1] Trace forward
    (bind (_locationout _normalout _hit) (CallFunction|TraceForward))
    ;[1 1 1] Was there a hit forward?
    (if _hit
      ;[1 1 1] Forward trace results to variables
      (Variables|Default|SetLocation _locationout)
      (Variables|Default|SetNormal _normalout)
      (else
        ;[1 1 1] Trace down
        (bind (_locationout_2 _normalout_2) (CallFunction|TraceDown))
        ;[1 1 1] Trace down hit results to variables
        (Variables|Default|SetLocation _locationout_2)
        (Variables|Default|SetNormal _normalout_2)))
    ;[1 1 1] Rotation from hit results and actor transform,
    (Transformation|SetWorldRotation (Variables|Default|GetArrow) (Math|Rotator|MakeRotfromXY (Variables|Default|GetNormal) (Math|Vector|RotateVector (Variables|Default|GetRightVector) (Math|Rotator|MakeRotator (Math|Random|RandomFloatinRangefromStream (* _noise -1.0) _noise (Variables|Default|GetStream)) (Math|Random|RandomFloatinRangefromStream (* _noise -1.0) _noise (Variables|Default|GetStream)) (Math|Random|RandomFloatinRangefromStream (* _noise -1.0) _noise (Variables|Default|GetStream))))) false false)
    ;[1 1 1] Location from hit results.
    (Transformation|SetWorldLocation (Variables|Default|GetArrow) (Variables|Default|GetLocation) false false)
    ;[1 1 1] Adding spline point
    (Spline|AddSplinePointatIndex (Variables|Default|GetSpline) (Variables|Default|GetLocation) _index "World" true))
  ;[1 1 1] Remove spline points from spline #2
  (Spline|ClearSplinePoints (Variables|Default|GetSpline1) true)
  ;[1 1 1] How many points for spline#2 ?
  (for _index_2 (range 0 (.ReturnValue (Math|Float|Division(WholeandRemainder) (Spline|GetSplineLength (Variables|Default|GetSpline)) (Variables|Default|GetMeshLenght))))
    ;[1 1 1] Add spline point to spline #2
    (Spline|AddSplinePointatIndex (Variables|Default|GetSpline1) (Spline|GetLocationatDistanceAlongSpline (Variables|Default|GetSpline) (* _index_2 (Variables|Default|GetMeshLenght)) "World") _index_2 "World" true))
  ;[1 1 1] Number of spline meshes
  (for _index_3 (range 0 (- (Spline|GetNumberOfSplinePoints (Variables|Default|GetSpline1)) 2))
    ;[1 1 1] Index and spline mesh to variables.
    (Variables|Default|SetCurrentIndex _index_3)
    (bind _returnvalue_2 (AddComponent|AddSplineMeshComponent false))
    (Variables|Default|SetCurrentSplineEMsh _returnvalue_2)
    ;[1 1 1] Set splineMeshand it's material
    (Components|StaticMesh|SetStaticMesh (Variables|Default|GetCurrentSplineEMsh) _mesh)
    (Rendering|Material|SetMaterial (Variables|Default|GetCurrentSplineEMsh) 0 (Rendering|Material|GetMaterial _mesh 0))
    ;[1 1 1] Mesh forward axis
    (SplineMesh|SetForwardAxis (Variables|Default|GetCurrentSplineEMsh) (Variables|Default|GetIn%20Forward%20Axis) true)
    ;[1 1 1] Set spline mesh start and end along spline #2
    (SplineMesh|SetStartandEnd (Variables|Default|GetCurrentSplineEMsh) (.Location (Spline|GetLocationandTangentatSplinePoint (Variables|Default|GetSpline1) (Variables|Default|GetCurrentIndex) "Local")) (.Tangent (Spline|GetLocationandTangentatSplinePoint (Variables|Default|GetSpline1) (Variables|Default|GetCurrentIndex) "Local")) (.Location (Spline|GetLocationandTangentatSplinePoint (Variables|Default|GetSpline1) (+ (Variables|Default|GetCurrentIndex) 1) "Local")) (.Tangent (Spline|GetLocationandTangentatSplinePoint (Variables|Default|GetSpline1) (+ (Variables|Default|GetCurrentIndex) 1) "Local")) true :!class /Script/Engine.SplineMeshComponent)
    ;[1 1 1] Scale spline mesh
    (SplineMesh|SetStartScale (Variables|Default|GetCurrentSplineEMsh) _returnvalue true :!class /Script/Engine.SplineMeshComponent)
    (SplineMesh|SetEndScale (Variables|Default|GetCurrentSplineEMsh) _returnvalue true :!class /Script/Engine.SplineMeshComponent)
    ;[1 1 1] Sqeeze first and last mesh
    (if (== (Variables|Default|GetCurrentIndex) 0)
      (SplineMesh|SetStartScale (Variables|Default|GetCurrentSplineEMsh) "(X=0.000000,Y=0.000000)" true :!class /Script/Engine.SplineMeshComponent))
    (if (== (Variables|Default|GetCurrentIndex) (- (Spline|GetNumberOfSplinePoints (Variables|Default|GetSpline1)) 2))
      (SplineMesh|SetEndScale (Variables|Default|GetCurrentSplineEMsh) "(X=0.000000,Y=0.000000)" true :!class /Script/Engine.SplineMeshComponent))))

(fn TraceForward
  (bind _arrow1 (Variables|Default|GetArrow1))
  ;[1 1 1] Trace results to variables
  (bind (_outhit _returnvalue) (Collision|LineTraceByChannel (+ (* (Math|Vector|GetForwardVector (Variables|Default|GetArrow)) (Variables|Default|GetTraceLength_UP)) (Transformation|GetWorldLocation (Variables|Default|GetArrow))) (+ (* (Math|Vector|RotateVectorAroundAxis (Math|Vector|GetUpVector _arrow1) (Variables|Default|GetLocalrotator) (Math|Vector|GetRightVector _arrow1)) (Variables|Default|GetTraceLength)) (Transformation|GetWorldLocation (Variables|Default|GetArrow))) "TraceTypeQuery1" true 0 "None"))
  (return (.Location (Collision|BreakHitResult _outhit)) (.Normal (Collision|BreakHitResult _outhit)) _returnvalue))

(fn TraceDown
  (bind _arrow2 (Variables|Default|GetArrow2))
  ;[1 1 1] trace results to variables
  (bind (_outhit _returnvalue) (Collision|LineTraceByChannel (+ (* (Math|Vector|GetForwardVector (Variables|Default|GetArrow1)) (Variables|Default|GetTraceLength)) (Transformation|GetWorldLocation (Variables|Default|GetArrow1))) (+ (* (Math|Vector|RotateVectorAroundAxis (Math|Vector|GetUpVector _arrow2) (Variables|Default|GetLocalrotator) (Math|Vector|GetRightVector _arrow2)) (Variables|Default|GetTraceLength)) (Transformation|GetWorldLocation (Variables|Default|GetArrow1))) "TraceTypeQuery1" true 0 "None"))
  (return (.Location (Collision|BreakHitResult _outhit)) (.Normal (Collision|BreakHitResult _outhit)) _returnvalue))