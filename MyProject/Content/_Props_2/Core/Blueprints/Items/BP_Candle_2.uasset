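; BP_Candle_2 is a candle item that takes matches as the item used on it.
; UseItem calls the parent and casts the item to BP_Matches, and CraftOrUseItem forwards to it after its own parent call.
; The IsFire check leads nowhere: the logic to decrement the match count, update the inventory and show Fire and Light is disconnected, so this graph never lights the candle.
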(fn ConstructionScript
  (|CallParentFunction))

(fn UseItem
  (params (Item :type Actor%20Object%20Reference))
  (|CallParentFunction Item)
  (bind _asbp_matches (Utilities|Casting|CastToBP_Matches Item))
  (if (not (Variables|Default|GetIsFire))
    _))

(fn CraftorUseItem
  (params (Item :type BP%20Base%20Item%20Object%20Reference))
  (|CallParentFunction Item)
  (CallFunction|UseItem Item))