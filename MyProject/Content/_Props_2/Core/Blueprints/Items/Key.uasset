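; Key item Blueprint that, once lit, acts as an igniter for doors and torches.
; CraftingEvent marks it used and on fire; its box overlap then calls FireSpyd on BP_Door2 or Fire on Torch2.
; CraftOrUseItem forwards to UseItem, which checks for BP_Matches but changes nothing itself, as its match-decrement and ignite logic is disconnected.
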(event OnComponentBeginOverlap(Box_0)
  (params (OverlappedComponent :type Primitive%20Component%20Object%20Reference) (OtherActor :type Actor%20Object%20Reference) (OtherComp :type Primitive%20Component%20Object%20Reference) (OtherBodyIndex :type Integer) (bFromSweep :type Boolean) (SweepResult :type Hit%20Result%20Structure%20%28by%20ref%29))
  (if (Variables|Default|GetIsFire)
    (bind _asbp_door_2 (Utilities|Casting|CastToBP_Door2 OtherActor)
      (:then
        (Default|FireSpyd _asbp_door_2))
      (:CastFailed
        (bind _astorch_2 (Utilities|Casting|CastToTorch2 OtherActor))
        (Default|Fire _astorch_2)))))

(event EventCraftingEvent
  (params (Condition :type Boolean) (Bp_baseitem :type BP%20Base%20Item%20Object%20Reference))
  (Variables|Default|SetUsed? true)
  (Variables|Default|SetIsFire true))

(fn ConstructionScript
  (|CallParentFunction))

(fn UseItem
  (params (Item :type Actor%20Object%20Reference))
  (|CallParentFunction Item)
  (bind _asbp_matches (Utilities|Casting|CastToBP_Matches Item))
  (if (not (Variables|Default|GetIsFire))
    _))

(fn CraftorUseItem
  (params (Item :type BP%20Base%20Item%20Object%20Reference))
  (|CallParentFunction Item)
  (CallFunction|UseItem Item))