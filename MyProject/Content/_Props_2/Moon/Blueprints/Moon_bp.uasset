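; Moon prop that renders a planet sphere with a parallax-detailed surface material lit by a referenced SunLight actor.
; The construction script picks a simple or masked shader, with a tessellated mesh and displacement at high quality, then sets its dynamic material parameters.
; Sun direction and colour, including colour temperature, are passed straight into the material.
; Tick runs only when live light updates are enabled.
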(event EventBeginPlay
  ;[1 1 1] Set tick
  (Actor|Tick|SetActorTickEnabled (or (Variables|Default|GetLiveUpdateLightDirection) (Variables|Default|GetLiveUpdateLightProperties)))
  (CallFunction|Refresh))

(event EventTick
  (params (DeltaSeconds :type Float%20%28single-precision%29))
  (if (Variables|Default|GetLiveUpdateLightDirection)
    (CallFunction|UpdateLightDirection))
  (if (Variables|Default|GetLiveUpdateLightProperties)
    (CallFunction|UpdateLightProperties)))

(fn ConstructionScript
  (bind _roughness (Variables|Default|GetRoughness))
  (bind _moonmasks (Variables|Default|GetMoonMasks))
  (bind _moonmap (Variables|Default|GetMoonMap))
  (bind _returnvalue (Utilities|IsValid _moonmasks))
  (bind _returnvalue_2 (* _roughness _roughness))
  (if (Variables|Default|GetHighQuality)
    ;[1 1 1] Create displacement dynamic material
    (Components|StaticMesh|SetStaticMesh (Variables|Default|GetMoon) "/Game/_Props_2/Moon/Objects/PlanetSphereTess_sm.PlanetSphereTess_sm")
    (bind _returnvalue_3 (Rendering|Material|CreateDynamicMaterialInstance (Variables|Default|GetMoon) 0 (select _returnvalue "/Game/_Props_2/Moon/Materials/MoonExtraDisplace_mat.MoonExtraDisplace_mat" "/Game/_Props_2/Moon/Materials/MoonDisplace_mat.MoonDisplace_mat") "None" :!class /Script/Engine.PrimitiveComponent))
    (Variables|Components|SetMoon%20Dynamic%20Material _returnvalue_3)
    (else
      ;[1 1 1] Create dynamic material
      (bind _returnvalue_4 (Rendering|Material|CreateDynamicMaterialInstance (Variables|Default|GetMoon) 0 (select _returnvalue "/Game/_Props_2/Moon/Materials/MoonExtra_mat.MoonExtra_mat" "/Game/_Props_2/Moon/Materials/Moon_mat.Moon_mat") "None" :!class /Script/Engine.PrimitiveComponent))
      (Variables|Components|SetMoon%20Dynamic%20Material _returnvalue_4)))
  (if _returnvalue
    ;[1 1 1] Parameters for complex shader
    (Rendering|Material|SetTextureParameterValue (Variables|Components|GetMoon%20Dynamic%20Material) "MaskMap" (Variables|Default|GetMoonMasks))
    (Rendering|Material|SetVectorParameterValue (Variables|Components|GetMoon%20Dynamic%20Material) "NightLights" (* (Utilities|ColourClamp (Variables|Default|GetEmissiveColourTint)) (Variables|Default|GetEmissiveIntensity)) :!class /Script/Engine.MaterialInstanceDynamic)
    (Rendering|Material|SetScalarParameterValue (Variables|Components|GetMoon%20Dynamic%20Material) "NightLightsTransition" (Variables|Default|GetDayNightTransition) :!class /Script/Engine.MaterialInstanceDynamic)
    (Rendering|Material|SetScalarParameterValue (Variables|Components|GetMoon%20Dynamic%20Material) "SpecIntensity" (Variables|Default|GetSpecIntensity) :!class /Script/Engine.MaterialInstanceDynamic)
    (else
      ;[1 1 1] Roughness for simple shader
      (Rendering|Material|SetScalarParameterValue (Variables|Components|GetMoon%20Dynamic%20Material) "A" (- 1.0 (* (/ _returnvalue_2 (+ _returnvalue_2 0.33)) 0.5)) :!class /Script/Engine.MaterialInstanceDynamic)
      (Rendering|Material|SetScalarParameterValue (Variables|Components|GetMoon%20Dynamic%20Material) "B" (* (/ _returnvalue_2 (+ _returnvalue_2 0.09)) 0.45) :!class /Script/Engine.MaterialInstanceDynamic)))
  (CallFunction|UpdateLightDirection)
  (CallFunction|UpdateLightProperties)
  (Rendering|Material|SetVectorParameterValue (Variables|Components|GetMoon%20Dynamic%20Material) "Fill" (* (Utilities|ColourClamp (Variables|Default|GetFillLightColour)) (Variables|Default|GetFillLightIntensity)) :!class /Script/Engine.MaterialInstanceDynamic)
  (Rendering|Material|SetScalarParameterValue (Variables|Components|GetMoon%20Dynamic%20Material) "ParallaxHeight" (* (Variables|Default|GetDetailHeight) 0.003) :!class /Script/Engine.MaterialInstanceDynamic)
  (Rendering|Material|SetScalarParameterValue (Variables|Components|GetMoon%20Dynamic%20Material) "ShadowSteps" (Variables|Default|GetShadowSteps) :!class /Script/Engine.MaterialInstanceDynamic)
  (Rendering|Material|SetScalarParameterValue (Variables|Components|GetMoon%20Dynamic%20Material) "ShadowPenumbra" (Variables|Default|GetShadowPenumbra) :!class /Script/Engine.MaterialInstanceDynamic)
  (Rendering|Material|SetScalarParameterValue (Variables|Components|GetMoon%20Dynamic%20Material) "MinSteps" (Variables|Default|GetParallaxMinSteps) :!class /Script/Engine.MaterialInstanceDynamic)
  (Rendering|Material|SetScalarParameterValue (Variables|Components|GetMoon%20Dynamic%20Material) "MaxSteps" (Variables|Default|GetParallaxMaxSteps) :!class /Script/Engine.MaterialInstanceDynamic)
  (Rendering|Material|SetScalarParameterValue (Variables|Components|GetMoon%20Dynamic%20Material) "Bounce" (* (Variables|Default|GetBounceLightIntensity) 0.5) :!class /Script/Engine.MaterialInstanceDynamic)
  (Rendering|Material|SetTextureParameterValue (Variables|Components|GetMoon%20Dynamic%20Material) "MoonMap" (select (Utilities|IsValid _moonmap) _moonmap (Variables|Default|GetNullMap)))
  (Rendering|Material|SetScalarParameterValue (Variables|Components|GetMoon%20Dynamic%20Material) "AmbientOcclusion" (Variables|Default|GetAmbientOcclusion) :!class /Script/Engine.MaterialInstanceDynamic)
  (Rendering|Material|SetScalarParameterValue (Variables|Components|GetMoon%20Dynamic%20Material) "NormalIntensity" (* (Variables|Default|GetNormalIntensity) (* (Math|Float|Power (* (* (Variables|Default|GetDetailHeight) 0.003) 0.22) 0.88) 2835.0)) :!class /Script/Engine.MaterialInstanceDynamic)
  (Rendering|Material|SetScalarParameterValue (Variables|Components|GetMoon%20Dynamic%20Material) "Dither" (Math|Float|SelectFloat 1.333 1.0 (Variables|Default|GetDither)) :!class /Script/Engine.MaterialInstanceDynamic)
  (Rendering|Material|SetScalarParameterValue (Variables|Components|GetMoon%20Dynamic%20Material) "TessellationMult" (Variables|Default|GetTessellationMultiplier) :!class /Script/Engine.MaterialInstanceDynamic))

(fn Refresh
  (CallFunction|UpdateLightDirection)
  (CallFunction|UpdateLightProperties))

(fn UpdateLightDirection
  (bind _sun_light (Variables|Default|GetSun%20Light))
  (Utilities|IsValid _sun_light
    (:Is%20Valid
      (Rendering|Material|SetVectorParameterValue (Variables|Components|GetMoon%20Dynamic%20Material) "SunForwardVector" (Math|Conversions|ToLinearColor(Vector) (* (Math|Vector|GetForwardVector (Transformation|GetWorldRotation (Variables|/Script/Engine.Light|GetLightComponent _sun_light))) -1)) :!class /Script/Engine.MaterialInstanceDynamic))))

(fn UpdateLightProperties
  (bind _returnvalue (Math|Trig|GetPI))
  (bind _sun_light (Variables|Default|GetSun%20Light))
  (bind _lightcomponent (Variables|/Script/Engine.Light|GetLightComponent _sun_light))
  (bind _returnvalue_2 (Rendering|Components|Light|GetLightColor _lightcomponent))
  (bind _intensity (Variables|/Script/Engine.LightComponentBase|GetIntensity _lightcomponent))
  (bind _returnvalue_3 (/ _intensity _returnvalue))
  (Utilities|IsValid _sun_light
    (:Is%20Valid
      ;[1 1 1] Update material parameter
      (Rendering|Material|SetVectorParameterValue (Variables|Components|GetMoon%20Dynamic%20Material) "SunlightIntensity" (Math|Color|SelectColor (* (* (Utilities|KelvintoRGB (Variables|/Script/Engine.LightComponent|GetTemperature _lightcomponent)) _returnvalue_2) _returnvalue_3) (* _returnvalue_2 _returnvalue_3) (Variables|/Script/Engine.LightComponent|GetbUseTemperature _lightcomponent)) :!class /Script/Engine.MaterialInstanceDynamic))))