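; BP_Bugs is an ambient prop that moves an animated skeletal mesh bug along a spline in an endless loop.
; BeginPlay applies the animation play rate and caches the spline length, and construction applies the bug scale.
; Tick advances the distance by a fixed, frame-rate-dependent Speed, snapping back to the start at the end.
; The bug follows the spline's world location, roll and yaw, with pitch held at zero.
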(event EventTick
  (params (DeltaSeconds :type Float%20%28single-precision%29))
  ;[1 1 1] Start after begin play finishes
  (if (Variables|Default|GetReady)
    ;[1 1 1] Reset position
    (if (<= (Variables|Default|GetDistanceAlongSpline) (- (Variables|Default|GetSplineLenght) 1.0))
      ;[1 1 1] Rotation and location along spline
      (bind _output_get (Variables|Default|SetDistanceAlongSpline (+ (Variables|Default|GetDistanceAlongSpline) (Variables|Default|GetSpeed))))
      (Transformation|SetWorldTransform (Variables|Default|GetSKM_Bug) (Math|Transform|MakeTransform (Spline|GetLocationatDistanceAlongSpline (Variables|Default|GetSpline) _output_get "World") (Math|Rotator|MakeRotator (.Roll (Math|Rotator|BreakRotator (Spline|GetRotationatDistanceAlongSpline (Variables|Default|GetSpline) _output_get "World"))) 0.0 (.Yaw (Math|Rotator|BreakRotator (Spline|GetRotationatDistanceAlongSpline (Variables|Default|GetSpline) _output_get "World")))) (Math|Conversions|ToVector(Float) (Variables|Default|GetBug%20Scale))) false false)
      (else
        (Variables|Default|SetDistanceAlongSpline 0.0)))))

(event EventBeginPlay
  ;[1 1 1] Animation playrate and spline lenght variable
  (Components|Timeline|SetPlayRate (Variables|Default|GetSKM_Bug) (Variables|Default|Getanimation%20PlayRate))
  (Variables|Default|SetSplineLenght (Spline|GetSplineLength (Variables|Default|GetSpline)))
  (Variables|Default|SetReady true))

(fn ConstructionScript
  (Transformation|SetWorldScale3D (Variables|Default|GetSKM_Bug) (Math|Conversions|ToVector(Float) (Variables|Default|GetBug%20Scale))))