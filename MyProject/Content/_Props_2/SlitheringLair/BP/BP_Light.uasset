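; BP_Light is a configurable flickering point light prop in the SlitheringLair prop set.
; The construction script applies exposed intensity, attenuation radius, shadow casting and color variables to the point light.
; On BeginPlay the Flicker timeline jumps to a random start time, so separate instances flicker out of sync.
; Each timeline update scales the base intensity by the flicker curve.
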(event EventBeginPlay
  (bind _flicker (Timeline|Flicker SetNewTime)
    (:Update
      (Rendering|Components|Light|SetIntensity (Variables|Default|GetPointLight) (* (Variables|Default|Getlight%20intensity) _flicker)))))

(fn ConstructionScript
  (bind _pointlight (Variables|Default|GetPointLight))
  (Rendering|Components|Light|SetIntensity _pointlight (Variables|Default|Getlight%20intensity))
  (Rendering|Lighting|SetAttenuationRadius _pointlight (Variables|Default|Getradius))
  (Rendering|Components|Light|SetCastShadows _pointlight (Variables|Default|Getcast%20shadows))
  (Rendering|Components|Light|SetLightColor _pointlight (Variables|Default|GetCLR) true))