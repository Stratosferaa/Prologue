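; BP_Vines is a Slithering Lair prop that scatters vine meshes procedurally over a configurable grid.
; Its Construction Script loops over rows times columns, adding one instance to each of two instanced mesh components per cell.
; The first mesh gets a location offset and random Y jitter, while the second stays on the grid point.
; Both get random yaw and scale; the event graph is empty.
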(event EventBeginPlay)

(event Collision|EventActorBeginOverlap
  (params (OtherActor :type Actor%20Object%20Reference)))

(event EventTick
  (params (DeltaSeconds :type Float%20%28single-precision%29)))

(fn ConstructionScript
  ;[1 1 1] Setting number of instances
  (for _index (range 0 (- (* (Variables|Meshes|Getrows) (Variables|Meshes|GetColumns)) 1))
    ;[1 1 1] Adding mesh instances
    (Components|InstancedStaticMesh|AddInstance (Variables|Default|GetMesh) (Math|Transform|MakeTransform (Math|Vector|MakeVector (.X (Math|Vector|BreakVector (+ (Variables|Meshes|Getslither%20Location%20offset) (.Location (Math|Transform|BreakTransform (Math|Conversions|ToTransform(Vector) (Math|Vector|MakeVector (Math|Conversions|ToFloat(Integer) (* (/ _index (Variables|Meshes|GetColumns)) (Variables|Meshes|GetMeshes%20distance%20Columns))) (Math|Conversions|ToFloat(Integer) (* (Math|Integer|%(Integer) _index (Variables|Meshes|GetColumns)) (Variables|Meshes|GetMeshes%20distance%20Rows))) 0.0))))))) (+ (.Y (Math|Vector|BreakVector (+ (Variables|Meshes|Getslither%20Location%20offset) (.Location (Math|Transform|BreakTransform (Math|Conversions|ToTransform(Vector) (Math|Vector|MakeVector (Math|Conversions|ToFloat(Integer) (* (/ _index (Variables|Meshes|GetColumns)) (Variables|Meshes|GetMeshes%20distance%20Columns))) (Math|Conversions|ToFloat(Integer) (* (Math|Integer|%(Integer) _index (Variables|Meshes|GetColumns)) (Variables|Meshes|GetMeshes%20distance%20Rows))) 0.0))))))) (* (Variables|Meshes|GetMax%20offset%20multiplier) (Math|Random|RandomFloatinRange 0.0 1e+01))) (.Z (Math|Vector|BreakVector (+ (Variables|Meshes|Getslither%20Location%20offset) (.Location (Math|Transform|BreakTransform (Math|Conversions|ToTransform(Vector) (Math|Vector|MakeVector (Math|Conversions|ToFloat(Integer) (* (/ _index (Variables|Meshes|GetColumns)) (Variables|Meshes|GetMeshes%20distance%20Columns))) (Math|Conversions|ToFloat(Integer) (* (Math|Integer|%(Integer) _index (Variables|Meshes|GetColumns)) (Variables|Meshes|GetMeshes%20distance%20Rows))) 0.0)))))))) (Math|Rotator|MakeRotator (.Roll (Math|Rotator|BreakRotator (.Rotation (Math|Transform|BreakTransform (Math|Conversions|ToTransform(Vector) (Math|Vector|MakeVector (Math|Conversions|ToFloat(Integer) (* (/ _index (Variables|Meshes|GetColumns)) (Variables|Meshes|GetMeshes%20distance%20Columns))) (Math|Conversions|ToFloat(Integer) (* (Math|Integer|%(Integer) _index (Variables|Meshes|GetColumns)) (Variables|Meshes|GetMeshes%20distance%20Rows))) 0.0)))))) (.Pitch (Math|Rotator|BreakRotator (.Rotation (Math|Transform|BreakTransform (Math|Conversions|ToTransform(Vector) (Math|Vector|MakeVector (Math|Conversions|ToFloat(Integer) (* (/ _index (Variables|Meshes|GetColumns)) (Variables|Meshes|GetMeshes%20distance%20Columns))) (Math|Conversions|ToFloat(Integer) (* (Math|Integer|%(Integer) _index (Variables|Meshes|GetColumns)) (Variables|Meshes|GetMeshes%20distance%20Rows))) 0.0)))))) (Math|Random|RandomFloatinRange 0.0 3.6e+02)) (* (* (.Scale (Math|Transform|BreakTransform (Math|Conversions|ToTransform(Vector) (Math|Vector|MakeVector (Math|Conversions|ToFloat(Integer) (* (/ _index (Variables|Meshes|GetColumns)) (Variables|Meshes|GetMeshes%20distance%20Columns))) (Math|Conversions|ToFloat(Integer) (* (Math|Integer|%(Integer) _index (Variables|Meshes|GetColumns)) (Variables|Meshes|GetMeshes%20distance%20Rows))) 0.0)))) (Math|Random|RandomFloatinRange 0.5 1.0)) (Variables|Meshes|GetScaling))))
    (Components|InstancedStaticMesh|AddInstance (Variables|Default|GetInstancedStaticMesh) (Math|Transform|MakeTransform (.Location (Math|Transform|BreakTransform (Math|Conversions|ToTransform(Vector) (Math|Vector|MakeVector (Math|Conversions|ToFloat(Integer) (* (/ _index (Variables|Meshes|GetColumns)) (Variables|Meshes|GetMeshes%20distance%20Columns))) (Math|Conversions|ToFloat(Integer) (* (Math|Integer|%(Integer) _index (Variables|Meshes|GetColumns)) (Variables|Meshes|GetMeshes%20distance%20Rows))) 0.0)))) (Math|Rotator|MakeRotator 0.0 0.0 (Math|Random|RandomFloatinRange 0.0 3.6e+02)) (Math|Conversions|ToVector(Float) (* (Math|Random|RandomFloatinRange 0.5 1.0) (Variables|Meshes|GetScaling)))))))