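; BP_HeightDisplay is a height marker that shows a size in meters through a scaled mesh and text labels.
; The construction script stretches the static mesh vertically by HeightM and raises it by half that height in centimeters.
; Two text renders, one for the value and one for the "m" unit, receive the same upward offset.
; The event graph holds no active logic.
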(event EventBeginPlay)

(event Collision|EventActorBeginOverlap
  (params (OtherActor :type Actor%20Object%20Reference)))

(event EventTick
  (params (DeltaSeconds :type Float%20%28single-precision%29)))

(fn ConstructionScript
  (bind _staticmesh (Variables|Default|GetStaticMesh))
  (bind _textrender (Variables|Default|GetTextRender))
  (bind _textrender2 (Variables|Default|GetTextRender2))
  (bind _output_get (Variables|Default|SetWorldOffset (Math|Vector|MakeVector 0.0 0.0 (/ (* (Variables|Default|GetHeight%20%28m%29) 1e+02) 2.0))))
  (Transformation|AddWorldOffset _staticmesh _output_get false false)
  (Transformation|SetWorldScale3D _staticmesh (Math|Vector|MakeVector 0.75 0.75 (Variables|Default|GetHeight%20%28m%29)))
  (Rendering|Components|TextRender|SetText _textrender (Utilities|Text|MakeLiteralText (Utilities|Text|ToText(Float) (Variables|Default|GetHeight%20%28m%29) "HalfToEven")))
  (Transformation|AddWorldOffset _textrender (Variables|Default|GetWorldOffset) false false)
  (Rendering|Components|TextRender|SetText _textrender2 (Utilities|Text|MakeLiteralText "m"))
  (Transformation|AddWorldOffset _textrender2 (Variables|Default|GetWorldOffset) false false))