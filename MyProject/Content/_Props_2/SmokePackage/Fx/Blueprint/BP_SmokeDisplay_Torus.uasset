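; Smoke display prop that shows a configurable Niagara smoke effect, named for a torus-shaped variant.
; The construction script assigns the Niagara asset to the SmokeFx component, resetting existing overrides, then pushes the Blueprint's variables into its user parameters.
; These parameters control color, lifetime, torus scale, particle size and spawning, velocity, vortex force and wind.
; The event graph has no active logic.
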(event EventBeginPlay)

(event Collision|EventActorBeginOverlap
  (params (OtherActor :type Actor%20Object%20Reference)))

(event EventTick
  (params (DeltaSeconds :type Float%20%28single-precision%29)))

(fn ConstructionScript
  (bind _smokefx (Variables|Default|GetSmokeFx))
  (Class|NiagaraComponent|SetAsset (Variables|Default|GetSmokeFx) (Variables|Default|GetNiagara) true)
  (Niagara|SetNiagaraVariable(LinearColor) _smokefx "Color" (Variables|Default|GetColor))
  (Niagara|SetNiagaraVariable(Float) _smokefx "LifeTime" (Variables|Default|GetLifeTime))
  (Niagara|SetNiagaraVariable(Float) _smokefx "TorusScale" (Variables|Default|GetTorusScale))
  (Niagara|SetNiagaraVariable(Float) _smokefx "InitialVelocity" (Variables|Default|GetInitialVelocity))
  (Niagara|SetNiagaraVariable(Float) _smokefx "ScaleColor" (Variables|Default|GetScaleColor))
  (Niagara|SetNiagaraVariable(Float) _smokefx "SmokeSize" (Variables|Default|GetSmokeSize))
  (Niagara|SetNiagaraVariable(Float) _smokefx "SpawnRate" (Variables|Default|GetSpawnRate))
  (Niagara|SetNiagaraVariable(Float) _smokefx "VortexForce" (Variables|Default|GetVortexForce))
  (Niagara|SetNiagaraVariable(Float) _smokefx "WindStrength" (Variables|Default|GetWindStrength))
  (Niagara|SetNiagaraVariable(Vector3) _smokefx "WindDirection" (Variables|Default|GetWindDirection)))